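; Elevator platform that moves along a two-point spline, up or down per UpElevator, when Character_BP steps into its box.
; Construction and BeginPlay set the spline, arrows and start position, while the parent class handles path movement.
; Leaving the box pauses or ends the path, depending on platform state.
; Intro and end sounds play on path changes, with a Tick countdown starting the loop sound after the intro's duration.
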(event `self.ReceiveBeginPlay`
  (`parent.ReceiveBeginPlay`)
  (`self.Initialization`))

(event `self.Box.OnComponentBeginOverlap`
  (params (OverlappedComponent :type "PrimitiveComponent Object Reference") (OtherActor :type "Actor Object Reference") (OtherComp :type "PrimitiveComponent Object Reference") (OtherBodyIndex :type Integer) (bFromSweep :type Boolean) (SweepResult :type "HitResult Structure (by ref)"))
  ;[1 1 1] Activate / Deactivate the elevator when the player enter/leave the box collider
  (cast `/Game/Blueprints/System/Character_BP` OtherActor)
  (set `self.PlatformCurrentState` "NewEnumerator1")
  (`self.BeginingPath`))

(event `self.Box.OnComponentEndOverlap`
  (params (OverlappedComponent :type "PrimitiveComponent Object Reference") (OtherActor :type "Actor Object Reference") (OtherComp :type "PrimitiveComponent Object Reference") (OtherBodyIndex :type Integer))
  ;[1 1 1] Activate / Deactivate the elevator when the player enter/leave the box collider
  (cast `/Game/Blueprints/System/Character_BP` OtherActor)
  (if (`|EnumEquality` (`self.PlatformCurrentState`) "NewEnumerator6")
    (`self.PausePath`)
    (else
      (`self.EndingPath`))))

(event `self.EndingPath`
  (`self.TryStartSound` "/Game/Sounds/Mechanics/Divided/MS_Elevator_End.MS_Elevator_End" 1.0 1.0)
  (set `self.ElapsedTimeBeforeLoopSound` 0.0)
  (if (`KismetMathLibrary.InRange_FloatFloat` (`self.AlphaPath`) 0.0 1.0 false false)
    (`parent.EndingPath`)
    (else
      (set `self.PlatformCurrentState` "NewEnumerator6"))))

(event `self.BeginingPath`
  (set `self.PauseTimeElapsed` 0.0)
  (`self.TryStartSound` "/Game/Sounds/Mechanics/Divided/MS_Elevator_Intro.MS_Elevator_Intro" 1.0 1.0)
  (set `self.ElapsedTimeBeforeLoopSound` (`SoundBase.Duration` (`AudioComponent.Sound` (`self.Audio`))))
  (`parent.BeginingPath`))

(event `self.ReceiveTick`
  (params (DeltaSeconds :type "Float (single-precision)"))
  (`parent.ReceiveTick` DeltaSeconds)
  (if (> (`self.ElapsedTimeBeforeLoopSound`) 0.0)
    (bind _output_get (set `self.ElapsedTimeBeforeLoopSound` (- (`self.ElapsedTimeBeforeLoopSound`) (`GameplayStatics.GetWorldDeltaSeconds`))))
    (if (<= _output_get 0.0)
      (`self.TryStartSound` "/Game/Sounds/Mechanics/Divided/MS_Elevator_Loop.MS_Elevator_Loop" 1.0 1.0))))

(fn `Initialization`
  (bind _toplocation (`self.TopLocation`))
  (bind _bottomlocation (`self.BottomLocation`))
  (bind (_returnvalue_inputkey _returnvalue_position) (break `SplinePoint` (`SplineComponent.GetSplinePointAt` (`self.Path`) 0 "Local")))
  (`SceneComponent.SetRelativeScale3D` (`self.Arrows`) (`KismetMathLibrary.MakeVector` 1.0 1.0 (`KismetMathLibrary.SelectFloat` -1.0 1.0 (`self.UpElevator`))))
  (`SplineComponent.SetSplinePoints` (`self.Path`) (select `bool` (`self.UpElevator`) :`false` (`|MakeArray` _toplocation _bottomlocation) :`true` (`|MakeArray` _bottomlocation _toplocation)) "Local" true)
  (`SceneComponent.K2_SetRelativeLocation` (`self.Moveable`) _returnvalue_position false false))

(fn `UserConstructionScript`
  (`parent.UserConstructionScript`)
  (`self.Initialization`))