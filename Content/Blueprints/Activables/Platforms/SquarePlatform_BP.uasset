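; SquarePlatform_BP is a square moving platform variant that adds sound and death-area control to its parent's path logic.
; On BeginPlay it starts a low-pitched platform MetaSound, and each tick it snaps the audio component to the Moveable's world location.
; When a path begins, the child-actor death area gets collision only if it is activated and the platform is in the designated death-area state.
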(event `self.ReceiveBeginPlay`
  (`parent.ReceiveBeginPlay`)
  (`self.TryStartSound` "/Game/Sounds/Mechanics/MS_SmallPlatform01.MS_SmallPlatform01" 0.5 0.4))

(event `self.BeginingPath`
  (`parent.BeginingPath`)
  (`self.SetActorEnableCollision` (`ChildActorComponent.ChildActor` (`self.BaseDeathArea_BP`)) (and (`self.IsDeathAreaActivate`) (`|EnumEquality` (`self.PlatformCurrentState`) (`self.DeathAreaState`)))))

(event `self.ReceiveTick`
  (params (DeltaSeconds :type "Float (single-precision)"))
  (`parent.ReceiveTick` DeltaSeconds)
  (`SceneComponent.K2_SetWorldLocation` (`self.Audio`) (`SceneComponent.K2_GetComponentLocation` (`self.Moveable`)) false false))

(fn `UserConstructionScript`
  (`parent.UserConstructionScript`))