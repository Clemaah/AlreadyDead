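; PressPlatform_BP is a press trap platform, a child Blueprint that adds sound and a toggled death area to its parent's path and activation logic.
; At each path start, it enables collision on the BaseDeathAreaBP child actor only in one platform state, choosing the metal trap sound for that same state.
; Activation runs the parent logic, then plays the metal trap sound.
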(event `self.BeginingPath`
  (bind _returnvalue (`|EnumEquality` (`self.PlatformCurrentState`) "NewEnumerator2"))
  (`parent.BeginingPath`)
  (`self.TryStartSound` (select `bool` _returnvalue :`true` "/Game/Sounds/Mechanics/SC_Metal_Trap.SC_Metal_Trap" :!type "SoundBase Object Reference") 1.0 1.0)
  (`self.SetActorEnableCollision` (`ChildActorComponent.ChildActor` (`self.BaseDeathArea_BP`)) _returnvalue))

(fn `Activation`
  (`parent.Activation`)
  (`self.TryStartSound` "/Game/Sounds/Mechanics/SC_Metal_Trap.SC_Metal_Trap" 1.0 1.0))

(fn `UserConstructionScript`
  (`parent.UserConstructionScript`))