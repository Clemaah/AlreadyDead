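; Base activable platform that moves its Moveable component along a spline path while in a specific activation state.
; Tick runs a moving/paused state machine that advances a normalized alpha by speed and pauses for a set duration at each end.
; After a pause, it either restarts from the beginning when looping or reverses direction, switching between forth and back ease functions.
; The eased alpha maps to a distance along the spline, which sets the world location.
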(event `self.ReceiveBeginPlay`
  (bind (_returnvalue_inputkey _returnvalue_position) (break `SplinePoint` (`SplineComponent.GetSplinePointAt` (`self.Path`) 0 "Local")))
  (`parent.ReceiveBeginPlay`)
  (set `self.PathLength` (`SplineComponent.GetSplineLength` (`self.Path`)))
  (set `self.CurrentEaseFunction` (`self.EaseFunctionForth`))
  (`SceneComponent.K2_SetRelativeLocation` (`self.Moveable`) _returnvalue_position false false))

(event `self.ReceiveTick`
  (params (DeltaSeconds :type "Float (single-precision)"))
  (`parent.ReceiveTick` DeltaSeconds)
  (if (`|EnumEquality` (`self.ActivableCurrentState`) "NewEnumerator2")
    (switch `/Game/Enums/CustomPlatformState_E` (`self.PlatformCurrentState`)
      (:`NewEnumerator2`
        (`self.ChangingAlpha` true)
        (`self.MovePlatform` :!label _label)
        (if (not (`KismetMathLibrary.InRange_FloatFloat` (`self.AlphaPath`) 0.0 1.0 false false))
          (`self.EndingPath`)))
      (:`NewEnumerator4`
        (`self.ChangingAlpha` false)
        (goto _label))
      (:`NewEnumerator1`
        (bind _output_get (set `self.PauseTimeElapsed` (- (`self.PauseTimeElapsed`) (`GameplayStatics.GetWorldDeltaSeconds`)) :!label _label_2))
        (if (<= _output_get 0.0)
          (`self.BeginingPath`)))
      (:`NewEnumerator7`
        (goto _label_2)))))

(event `EndingPath`
  (`self.PausePath`))

(event `PausePath`
  (set `self.PlatformCurrentState` (select `bool` (or (`|EnumEquality` (`self.PlatformCurrentState`) "NewEnumerator2") (`|EnumEquality` (`self.PlatformCurrentState`) "NewEnumerator6")) :`false` "NewEnumerator1" :`true` "NewEnumerator7" :!type "/Game/Enums/CustomPlatformState_E Enum"))
  (set `self.PauseTimeElapsed` (`self.PauseDuration`)))

(event `BeginingPath`
  (if (`self.IsLooping`)
    (set `self.AlphaPath` 0.0)
    (set `self.PlatformCurrentState` "NewEnumerator2")
    (elif (`|EnumEquality` (`self.PlatformCurrentState`) "NewEnumerator1")
      (set `self.PlatformCurrentState` "NewEnumerator2")
      (set `self.CurrentEaseFunction` (`self.EaseFunctionForth`))
      (else
        (set `self.PlatformCurrentState` "NewEnumerator4")
        (set `self.CurrentEaseFunction` (`self.EaseFunctionBack`))))))

(fn `ChangingAlpha`
  (params (IsGoingForward :type Boolean))
  (bind _returnvalue (* (`GameplayStatics.GetWorldDeltaSeconds`) (/ (`self.Speed`) 100.0)))
  (set `self.AlphaPath` (`KismetMathLibrary.FClamp` (+ (`self.AlphaPath`) (`KismetMathLibrary.SelectFloat` _returnvalue (* _returnvalue -1.0) IsGoingForward)))))

(fn `MovePlatform`
  (`SceneComponent.K2_SetWorldLocation` (`self.Moveable`) (`SplineComponent.GetLocationAtDistanceAlongSpline` (`self.Path`) (`|EaseFunction` (`self.CurrentEaseFunction`) (`self.AlphaPath`) 0.0 (`self.PathLength`) (`self.EaseIntensity`) 1) "World") false false))

(fn `UserConstructionScript`
  (`parent.UserConstructionScript`))