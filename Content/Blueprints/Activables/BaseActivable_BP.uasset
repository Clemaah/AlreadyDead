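; Base Blueprint for activables that a linked activator switches between Deactivated, Delayed and Activated states.
; BeginPlay applies the default state and binds to the activator's trigger delegate.
; Triggering a deactivated activable starts a Tick-driven timer that activates it once the activation delay elapses; triggering an activated one deactivates it only if allowed.
; Each transition calls SwitchBehaviour, and IsOn also counts Delayed as on.
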(event `self.ReceiveBeginPlay`
  (`parent.ReceiveBeginPlay`)
  ;[1 1 1] Variables initialization
  (set `self.ActivableCurrentState` (`self.DefaultState`))
  (bind _activator (`self.Activator`)
    (:`then`
      (add `/Game/Blueprints/Triggers/Activators/BaseActivator_BP.TriggerActivablesDelegate` _activator (`|CreateDelegate` :!event `TrySwitchActivableState`)))
    (:`else`)))

(event `TrySwitchActivableState`
  ;[1 1 1] Event call when the linked activator is used. Change the Activable state.
  (switch `/Game/Enums/CustomActivableState_E` (`self.ActivableCurrentState`)
    (:`NewEnumerator2`
      (if (`self.CanBeDeactivated`)
        (set `self.ActivableCurrentState` "NewEnumerator1")
        (`self.SwitchBehaviour`)))
    (:`NewEnumerator1`
      (set `self.TimerActivation` 0.0)
      (set `self.ActivableCurrentState` "NewEnumerator3")
      (`self.SwitchBehaviour`))))

(event `self.ReceiveTick`
  (params (DeltaSeconds :type "Float (single-precision)"))
  ;[1 1 1] Tick event
  (`parent.ReceiveTick` DeltaSeconds)
  (if (`|EnumEquality` (`self.ActivableCurrentState`) "NewEnumerator3")
    (bind _output_get (set `self.TimerActivation` (+ DeltaSeconds (`self.TimerActivation`))))
    (if (>= _output_get (`self.ActivationDelay`))
      (`self.Activation`)
      (`self.SwitchBehaviour`))))

(fn `Activation`
  (set `self.ActivableCurrentState` "NewEnumerator2"))

(fn `IsOn`
  (returns (IsOn :type Boolean))
  (return (and (`parent.IsOn`) (`|EnumInequality` (`self.ActivableCurrentState`) "NewEnumerator1"))))

(fn `UserConstructionScript`)