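; Activable crane that, when switched on, plays a sound and yaws its Moveable component by TotalRotation along a timeline, stopping when switched off.
; Each update also orbits attached actors, recursively, around the crane's pivot by the yaw delta.
; Timeline play rate comes from separate forward and backward durations, swapped as direction flips on finish.
; In round-trip mode it reverses after a pause, otherwise it updates its activable state.
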(event `self.ReceiveBeginPlay`
  (`parent.ReceiveBeginPlay`)
  (`self.SetAnimationDuration` (`self.ForwardDuration`)))

(event `Event OnRoundTripReverse`
  (`KismetSystemLibrary.Delay` (`self.PauseDuration`))
  (bind (_direction _alpharotation) (`Timeline|Timeline` :!via `Reverse`)
    (:`Update`
      (`self.UpdateRotation` _alpharotation))
    (:`Finished`
      (`self.SwichTimelineDirection`)
      (if (and (not (`self.IsGoingForward`)) (`self.IsDoingRoundTrip`))
        (`self.Event OnRoundTripReverse`)
        (else
          (set `self.ActivableCurrentState` "NewEnumerator1"))))))

(event `self.SwitchBehaviour`
  (`parent.SwitchBehaviour`)
  (if (`self.IsOn`)
    (`self.TryStartSound` "/Game/Sounds/Mechanics/MS_Grues.MS_Grues" 0.7 1.0)
    (if (`self.IsGoingForward`)
      (`TimelineComponent.Play` (`self.Timeline`))
      (else
        (`TimelineComponent.Reverse` (`self.Timeline`))))
    (else
      (`TimelineComponent.Stop` (`self.Timeline`)))))

(fn `RotateLinkActor`
  (params (LinkedActor :type "Actor Object Reference") (Alpha :type "Float (double-precision)"))
  (locals (CurrentRotationOffset :type "Float (double-precision)") (CurrentAn :type "Float (double-precision)"))
  (bind _returnvalue (`self.K2_GetActorLocation`))
  (bind (_relativerotation_roll _relativerotation_pitch _relativerotation_yaw) (`KismetMathLibrary.BreakRotator` (`SceneComponent.RelativeRotation` (`self.Moveable`))))
  (bind _returnvalue_2 (- (* Alpha (`self.TotalRotation`)) _relativerotation_yaw))
  (set `local.CurrentRotationOffset` _returnvalue_2)
  (`self.K2_SetActorLocation` (`local.LinkedActor`) (+ (`KismetMathLibrary.RotateAngleAxis` (- (`self.K2_GetActorLocation` (`local.LinkedActor`)) _returnvalue) _returnvalue_2 (0.0 0.0 1.0)) _returnvalue) false false)
  (`self.K2_AddActorWorldRotation` (`local.LinkedActor`) (`KismetMathLibrary.MakeRotator` 0.0 0.0 (`local.CurrentRotationOffset`)) false false))

(fn `SetAnimationDuration`
  (params (Duration :type "Float (double-precision)"))
  (`TimelineComponent.SetPlayRate` (`self.Timeline`) (/ 1.0 Duration)))

(fn `SwichTimelineDirection`
  (bind _output_get (set `self.IsGoingForward` (not (`self.IsGoingForward`))))
  (if _output_get
    (`self.SetAnimationDuration` (`self.ForwardDuration`))
    (else
      (`self.SetAnimationDuration` (`self.BackwardDuration`)))))

(fn `UpdateRotation`
  (params (TimelineValue :type "Float (double-precision)"))
  (for _array_element (`self.GetAttachedActors` true true)
    (`self.RotateLinkActor` _array_element TimelineValue))
  (`SceneComponent.K2_SetRelativeRotation` (`self.Moveable`) (`KismetMathLibrary.RLerp` (struct) (`KismetMathLibrary.MakeRotator` 0.0 0.0 (`self.TotalRotation`)) TimelineValue true) false false))

(fn `UserConstructionScript`
  (`parent.UserConstructionScript`))