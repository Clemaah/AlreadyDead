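; Activable turbine actor that spins continuously and plays a turbine engine sound, built on a parent activable class.
; Every tick it adds a local yaw rotation scaled by RotationSpeed and delta time, with no state check in this Blueprint.
; The engine sound starts on activation, or at BeginPlay when the activable's current state already matches a specific enum value.
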(event `self.ReceiveBeginPlay`
  (`parent.ReceiveBeginPlay`)
  (if (`|EnumEquality` (`self.ActivableCurrentState`) "NewEnumerator2")
    (`self.TryStartSound` "/Game/Sounds/Mechanics/MS_Engine_Turbine.MS_Engine_Turbine" 0.6 0.9)))

(event `self.ReceiveTick`
  (params (DeltaSeconds :type "Float (single-precision)"))
  ;[1 1 1] Tick Event
  (`parent.ReceiveTick` DeltaSeconds)
  (`self.Rotation`))

(fn `Activation`
  (`parent.Activation`)
  (`self.TryStartSound` "/Game/Sounds/Mechanics/MS_Engine_Turbine.MS_Engine_Turbine" 0.6 0.9))

(fn `Rotation`
  (bind (_returnvalue_roll _returnvalue_pitch _returnvalue_yaw) (`KismetMathLibrary.BreakRotator` (`KismetMathLibrary.MakeRotator` 0.0 0.0 (`self.RotationSpeed`))))
  (`self.K2_AddActorLocalRotation` (`KismetMathLibrary.MakeRotator` 0.0 0.0 (* _returnvalue_yaw (`GameplayStatics.GetWorldDeltaSeconds`)))))

(fn `UserConstructionScript`)