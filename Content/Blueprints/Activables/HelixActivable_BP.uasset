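; Activable helix, apparently a ventilation fan, that spins and switches a box collider with its on/off state.
; Extends the parent activable's switch behaviour to enable query and physics collision on the Box only while on.
; Tick applies a frame-rate-independent local pitch rotation from RotationSpeed, with no state check of its own.
; The ventilation MetaSound starts on Activation, or at BeginPlay if the initial state matches.
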(event `self.ReceiveBeginPlay`
  (`parent.ReceiveBeginPlay`)
  (if (`|EnumEquality` (`self.ActivableCurrentState`) "NewEnumerator2")
    (`self.TryStartSound` "/Game/Sounds/Mechanics/MS_Ventillation.MS_Ventillation" 1.5 1.0)))

(event `self.SwitchBehaviour`
  ;[1 1 1] Activation/Deactivation of the collider
  (`parent.SwitchBehaviour`)
  (`PrimitiveComponent.SetCollisionEnabled` (`self.Box`) (select `bool` (`self.IsOn`) :`false` "NoCollision" :`true` "QueryAndPhysics" :!type "ECollisionEnabled Enum")))

(event `self.ReceiveTick`
  (params (DeltaSeconds :type "Float (single-precision)"))
  ;[1 1 1] Tick Event
  (`parent.ReceiveTick` DeltaSeconds)
  (`self.Rotation`))

(fn `Activation`
  (`parent.Activation`)
  (`self.TryStartSound` "/Game/Sounds/Mechanics/MS_Ventillation.MS_Ventillation" 1.5 1.0))

(fn `Rotation`
  (bind (_returnvalue_roll _returnvalue_pitch) (`KismetMathLibrary.BreakRotator` (`KismetMathLibrary.MakeRotator` 0.0 (`self.RotationSpeed`))))
  (`self.K2_AddActorLocalRotation` (`KismetMathLibrary.MakeRotator` 0.0 (* _returnvalue_pitch (`GameplayStatics.GetWorldDeltaSeconds`)))))

(fn `UserConstructionScript`)