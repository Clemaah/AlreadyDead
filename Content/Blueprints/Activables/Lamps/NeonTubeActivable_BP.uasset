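; Neon tube lamp, a child of an activable parent Blueprint, that lights up or goes dark with its activation state.
; It overrides the parent's SwitchBehaviour event, calling the parent version first.
; It then checks the current state to set the point light to its area intensity or zero and to swap the tube mesh between activated and deactivated materials.
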(event `/Game/Blueprints/BaseGPE_BP.SwitchBehaviour`
  (bind _returnvalue (`|EnumEquality` (`self.ActivableCurrentState`) "NewEnumerator2"))
  (`parent.SwitchBehaviour`)
  ;[1 1 1] Switch intensity and material when activated.
  (`LightComponent.SetIntensity` (`self.PointLight2`) (`KismetMathLibrary.SelectFloat` (`self.AreaIntensity`) 0.0 _returnvalue))
  (`PrimitiveComponent.SetMaterial` (`self.Tube`) 0 (select `bool` _returnvalue :`false` (`self.DeactivatedMaterial`) :`true` (`self.ActivatedMaterial`))))

(fn `UserConstructionScript`
  (`parent.UserConstructionScript`))