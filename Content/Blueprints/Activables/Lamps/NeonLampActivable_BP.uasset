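; Neon lamp activable that switches its lights and tube materials with its activation state.
; It overrides the parent's SwitchBehaviour event, calls the parent version, then checks the current activable state.
; When activated, the spot and point lights take their configured intensities and both tubes get the activated material.
; Any other state zeroes both lights and applies the deactivated material.
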(event `/Game/Blueprints/BaseGPE_BP.SwitchBehaviour`
  (`parent.SwitchBehaviour`)
  (if (`|EnumEquality` (`self.ActivableCurrentState`) "NewEnumerator2")
    ;[1 1 1] Changing intensity and material when activated.
    (`LightComponent.SetIntensity` (`self.SpotLight`) (`self.Intensity`))
    (`LightComponent.SetIntensity` (`self.PointLight`) (`self.AreaIntensity`))
    (`PrimitiveComponent.SetMaterial` (`self.Tube1`) 0 (`self.ActivatedMaterial`))
    (`PrimitiveComponent.SetMaterial` (`self.Tube2`) 0 (`self.ActivatedMaterial`))
    (else
      (`LightComponent.SetIntensity` (`self.SpotLight`) 0.0)
      (`LightComponent.SetIntensity` (`self.PointLight`) 0.0)
      (`PrimitiveComponent.SetMaterial` (`self.Tube1`) 0 (`self.DeactivatedMaterial`))
      (`PrimitiveComponent.SetMaterial` (`self.Tube2`) 0 (`self.DeactivatedMaterial`)))))

(fn `UserConstructionScript`
  (`parent.UserConstructionScript`))