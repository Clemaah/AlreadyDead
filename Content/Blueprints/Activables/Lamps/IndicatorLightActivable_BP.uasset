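; IndicatorLightActivable_BP is an activable indicator lamp that shows its on or off state through color.
; It overrides the parent's SwitchBehaviour event, calling the parent first and then checking the current activable state.
; Both point lights and the glass mesh's material swap between activated and deactivated color and material variants to match that state.
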(event `/Game/Blueprints/BaseGPE_BP.SwitchBehaviour`
  (`parent.SwitchBehaviour`)
  (if (`|EnumEquality` (`self.ActivableCurrentState`) "NewEnumerator2")
    ;[1 1 1] Changing light color and material when activated.
    (`LightComponent.SetLightColor` (`self.PointLight1`) (`self.ActivatedColor`) true)
    (`LightComponent.SetLightColor` (`self.PointLight2`) (`self.ActivatedColor`) true)
    (`PrimitiveComponent.SetMaterial` (`self.Glass`) 0 (`self.ActivatedMaterial`))
    (else
      (`LightComponent.SetLightColor` (`self.PointLight1`) (`self.DeactivatedColor`) true)
      (`LightComponent.SetLightColor` (`self.PointLight2`) (`self.DeactivatedColor`) true)
      (`PrimitiveComponent.SetMaterial` (`self.Glass`) 0 (`self.DeactivatedMaterial`)))))

(fn `UserConstructionScript`
  (`parent.UserConstructionScript`))