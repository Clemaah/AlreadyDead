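; Base Blueprint for activable lamps, handling the sound they make when switched on.
; Activation runs the parent logic, plays a light switch sound and stores that sound's duration as a countdown.
; Tick decrements the countdown through LoopDelayBehaviour and starts the neon loop sound once it runs out, so the hum follows the click.
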(event `self.ReceiveTick`
  (params (DeltaSeconds :type "Float (single-precision)"))
  (`parent.ReceiveTick` DeltaSeconds)
  (if (> (`self.ElapsedTimeBeforeLoopSound`) 0.0)
    (bind _output_get (set `self.ElapsedTimeBeforeLoopSound` (- (`self.ElapsedTimeBeforeLoopSound`) (`GameplayStatics.GetWorldDeltaSeconds`))))
    (if (<= _output_get 0.0)
      (`self.TryStartSound` "/Game/Sounds/Mechanics/MS_Neon_Loop.MS_Neon_Loop" (`self.VolumeLoop`) (`self.PitchLoop`)))))

(fn `Activation`
  (`parent.Activation`)
  (`self.TryStartSound` "/Game/Sounds/Mechanics/MS_Light_Switch.MS_Light_Switch" (`self.VolumeActivate`) (`self.PitchActivate`))
  (set `self.ElapsedTimeBeforeLoopSound` (`SoundBase.Duration` (`AudioComponent.Sound` (`self.Audio`)))))

(fn `UserConstructionScript`
  (`parent.UserConstructionScript`))