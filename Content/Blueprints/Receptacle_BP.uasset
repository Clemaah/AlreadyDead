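; Receptacle Blueprint that can be toggled between activated and deactivated states, with matching visual feedback.
; SwitchActivation flips IsActivated, then uses it to drive the Niagara effect, the point light's visibility and the material on the Cylinder4 component.
; The construction script only calls its parent, and nothing in this Blueprint calls the toggle itself.
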(fn `SwitchActivation`
  (bind _output_get (set `self.IsActivated` (not (`self.IsActivated`))))
  (`ActorComponent.SetActive` (`self.Niagara`) _output_get false)
  (`SceneComponent.SetVisibility` (`self.PointLight`) _output_get false)
  (`PrimitiveComponent.SetMaterial` (`self.Cylinder4`) 0 (select `bool` _output_get :`false` (`self.DeactivatedMaterial`) :`true` (`self.ActivatedMaterial`) :!type "MaterialInterface Object Reference")))

(fn `UserConstructionScript`
  (`parent.UserConstructionScript`))