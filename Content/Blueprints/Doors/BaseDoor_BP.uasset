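; Base door puzzle where the player must press the correct key lockers among a set of linked Lockers to unlock it.
; Locker delegates feed a press counter; once presses match the key count, locker states are validated, leading to success or error feedback.
; Tick runs two countdowns: an optional unlock limit with ticking audio and player UI timer, and a delay that resets lockers after failure or timeout.
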(event `self.ReceiveBeginPlay`
  (`parent.ReceiveBeginPlay`)
  (for _array_element (`self.Lockers`)
    (add `/Game/Blueprints/Triggers/Activators/Lockers/BaseLocker_BP.TriggerDoorDelegate` _array_element (`|CreateDelegate` :!event `OnKeyPressed`))
    (if (`/Game/Blueprints/Triggers/Activators/Lockers/BaseLocker_BP.IsKey` _array_element)
      (`/Engine/EditorBlueprintResources/StandardMacros.IncrementInt` (`self.AmoutOfKeys`)))))

(event `OnKeyPressed`
  (if (not (`self.IsUnlockingDoor`))
    (bind _result (`/Engine/EditorBlueprintResources/StandardMacros.IncrementInt` (`self.AmountOfPressedLockers`))
      (:`  `
        (if (== _result (`self.AmoutOfKeys`))
          (set `self.IsUnlockingDoor` true)
          (`self.TryUnlockingDoor`)
          (elif (== (`self.AmountOfPressedLockers`) 1)
            (bind _output_get (set `self.ElapsedUnlockTime` (`self.UnlockDelay`)))
            (if (> _output_get 0.0)
              (set `AudioComponent.AttenuationSettings` null (`self.Audio`))
              (`self.TryStartSound` "/Game/Sounds/Mechanics/SC_M_TickingClock_Cue.SC_M_TickingClock_Cue" 1.0 1.0 true)
              (`self.ToggleTimerWidget` true))))))))

(event `self.ReceiveTick`
  (params (DeltaSeconds :type "Float (single-precision)"))
  (bind _elapsedunlocktime (`self.ElapsedUnlockTime`))
  (`parent.ReceiveTick` DeltaSeconds)
  (`|ExecutionSequence`
    (:`then_0`
      (if (> (`self.ElapsedUnlockTime`) 0.0)
        (`/Game/UI/WB_Interface.UpdateTimer` (`self.GetInterface`) _elapsedunlocktime)
        (bind _output_get (set `self.ElapsedUnlockTime` (- _elapsedunlocktime DeltaSeconds)))
        (if (<= _output_get 0.0)
          (`AudioComponent.SetSound` (`self.Audio`) null)
          (`self.InvalidateKeys`))))
    (:`then_1`
      (`|ExecutionSequence`
        (:`then_0`
          (if (> (`self.ElapsedInvalidateTime`) 0.0)
            (bind _output_get_2 (set `self.ElapsedInvalidateTime` (- (`self.ElapsedInvalidateTime`) DeltaSeconds)))
            (if (<= _output_get_2 0.0)
              (`self.ResetKeys`))))))))

(event `self.SwitchBehaviour`
  (`parent.SwitchBehaviour`)
  (if (not (== (`self.UnlockDelay`) 0.0))
    (`/Game/UI/WB_Interface.ToggleFreeze` (`self.GetInterface`) (`self.IsFreezedByWord`))))

(fn `GetInterface`
  (returns (Interface :type "/Game/UI/WB_Interface Object Reference"))
  (bind _ascharacter_bp (cast `/Game/Blueprints/System/Character_BP` (`GameplayStatics.GetPlayerCharacter` 0)))
  (return (`/Game/Blueprints/System/Character_BP.Interface` _ascharacter_bp)))

(fn `InvalidateKeys`
  (`self.ToggleTimerWidget` false)
  (for _array_element (`self.Lockers`)
    (`/Game/Blueprints/Triggers/Activators/Lockers/BaseLocker_BP.ChangeLockerState` _array_element "NewEnumerator0"))
  (set `self.ElapsedInvalidateTime` (`self.InvalidateDelay`))
  (`GameplayStatics.PlaySound2D` "/Game/Sounds/Mechanics/MS_ErrorCode.MS_ErrorCode" 0.4 1.0 0.0 null null)
  (`self.TryPauseSound`))

(fn `IsCodeValid`
  (returns (Validity :type Boolean))
  (locals (Valid :type Boolean :default true))
  (set `local.Valid` true)
  (for _array_element (`self.Lockers`)
    (if (xor (`|EnumEquality` (`/Game/Blueprints/Triggers/Activators/Lockers/BaseLocker_BP.LockerCurrentState` _array_element) "NewEnumerator2") (`/Game/Blueprints/Triggers/Activators/Lockers/BaseLocker_BP.IsKey` _array_element))
      (set `local.Valid` false)
      (break)))
  (return (`local.Valid`)))

(fn `ResetKeys`
  (for _array_element (`self.Lockers`)
    (`/Game/Blueprints/Triggers/Activators/Lockers/BaseLocker_BP.ChangeLockerState` _array_element "NewEnumerator3"))
  (set `self.AmountOfPressedLockers` 0)
  (set `self.IsUnlockingDoor` false))

(fn `ToggleTimerWidget`
  (params (Activate :type Boolean))
  (if (> (`self.UnlockDelay`) 0.0)
    (`/Game/UI/WB_Interface.DisplayTimer` (`self.GetInterface`) Activate)))

(fn `TryUnlockingDoor`
  (set `self.ElapsedUnlockTime` 0.0)
  (set `self.AmountOfPressedLockers` 0)
  (if (`self.IsCodeValid`)
    (`self.UnlockDoor`)
    (else
      (`self.InvalidateKeys`))))

(fn `UnlockDoor`
  (`self.ToggleTimerWidget` false)
  (set `self.ElapsedUnlockTime` 0.0)
  (for _array_element (`self.Lockers`)
    (`/Game/Blueprints/Triggers/Activators/Lockers/BaseLocker_BP.ChangeLockerState` _array_element (select `bool` (`/Game/Blueprints/Triggers/Activators/Lockers/BaseLocker_BP.IsKey` _array_element) :`false` "NewEnumerator4" :`true` "NewEnumerator1" :!type "/Game/Enums/CustomLockerState_E Enum")))
  (if (`self.ActivateSuccessSound`)
    (`GameplayStatics.PlaySound2D` "/Game/Sounds/Mechanics/MS_SucessCode.MS_SucessCode" 0.15 1.0 0.0 null null)))

(fn `UserConstructionScript`)