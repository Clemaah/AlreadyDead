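; Thin door Blueprint, a child of a lockable door, that slides its Top and Bottom parts toward target positions when unlocked.
; UnlockDoor resets an elapsed timer, plays the door sound and switches the emissive pieces to the open material.
; Tick lerps each part from its current location using a float curve until OpeningDelay elapses.
; BeginPlay presets the timer to that delay, keeping the animation idle.
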(event `self.ReceiveBeginPlay`
  (`parent.ReceiveBeginPlay`)
  (set `self.ElapsedOpeningTime` (`self.OpeningDelay`)))

(event `self.UnlockDoor`
  (bind _openmaterial (`self.OpenMaterial`))
  (`parent.UnlockDoor`)
  (set `self.ElapsedOpeningTime` 0.0)
  (`self.TryStartSound` "/Game/Sounds/Mechanics/MS_Door.MS_Door" 1.0 1.0)
  (`PrimitiveComponent.SetMaterial` (`self.EmissiveHalfCylinderFull1`) 0 _openmaterial)
  (`PrimitiveComponent.SetMaterial` (`self.EmissiveBorder1`) 0 _openmaterial)
  (`PrimitiveComponent.SetMaterial` (`self.EmissiveBorder2`) 0 _openmaterial)
  (`PrimitiveComponent.SetMaterial` (`self.EmissiveBorder3`) 0 _openmaterial)
  (`PrimitiveComponent.SetMaterial` (`self.EmissiveBorder4`) 0 _openmaterial)
  (`PrimitiveComponent.SetMaterial` (`self.EmissiveHalfCylinderFull2`) 0 _openmaterial))

(event `self.ReceiveTick`
  (params (DeltaSeconds :type "Float (single-precision)"))
  (`parent.ReceiveTick` DeltaSeconds)
  (`|ExecutionSequence`
    (:`then_0`
      (if (< (`self.ElapsedOpeningTime`) (`self.OpeningDelay`))
        (bind _output_get (set `self.ElapsedOpeningTime` (+ (`self.ElapsedOpeningTime`) DeltaSeconds)))
        (bind _returnvalue (`CurveFloat.GetFloatValue` (`self.OpeningCurve`) _output_get))
        (`self.AnimateDoor` (`self.Top`) (`self.TargetUp`) _returnvalue)
        (`self.AnimateDoor` (`self.Bottom`) (`self.TargetDown`) _returnvalue)))))

(fn `AnimateDoor`
  (params (Object :type "SceneComponent Object Reference") (Target :type "SceneComponent Object Reference") (Alpha :type "Float (single-precision)"))
  (`SceneComponent.K2_SetWorldLocation` Object (`KismetMathLibrary.VLerp` (`SceneComponent.K2_GetComponentLocation` Object) (`SceneComponent.K2_GetComponentLocation` Target) Alpha) false false))

(fn `UserConstructionScript`
  (`parent.UserConstructionScript`))