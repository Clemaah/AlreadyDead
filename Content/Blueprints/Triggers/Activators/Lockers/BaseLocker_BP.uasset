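; Base locker trigger Blueprint that fires activable and door delegates, set off either by player contact or by interaction.
; It overrides its parents' range and interact events, switching an enum state only from one specific value.
; ChangeLockerState fires the activables, then the door after a short delay, and re-fires the activables on one reverse transition.
; The character's interaction prompt toggles only in the usable state.
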(event `self.PlayerInRange`
  (params (OverlappedComponent :type "PrimitiveComponent Object Reference") (OtherActor :type "Actor Object Reference") (OtherComp :type "PrimitiveComponent Object Reference") (OtherBodyIndex :type Integer) (bFromSweep :type Boolean) (SweepResult :type "HitResult Structure (by ref)"))
  (`parent.PlayerInRange` OverlappedComponent OtherActor OtherComp OtherBodyIndex bFromSweep SweepResult)
  (if (`self.IsActivatedByContact`)
    (if (`|EnumEquality` (`self.LockerCurrentState`) "NewEnumerator3") :!label _label
      (`self.ChangeLockerState` "NewEnumerator2"))))

(event `self.Interact`
  (`parent.Interact`)
  (if (not (`self.IsActivatedByContact`))
    (`self.ToggleWidget` false)
    (goto _label)))

(event `ChangeLockerState`
  (params (NewState :type "/Game/Enums/CustomLockerState_E Enum" :default "NewEnumerator3"))
  (if (`|EnumEquality` NewState "NewEnumerator2")
    (set `self.LockerCurrentState` NewState)
    (`self.TriggerActivablesDelegate`)
    (`KismetSystemLibrary.Delay` 0.1)
    (`self.TriggerDoorDelegate`)
    (else
      (if (and (`|EnumEquality` NewState "NewEnumerator0") (`|EnumEquality` (`self.LockerCurrentState`) "NewEnumerator2"))
        (`self.TriggerActivablesDelegate`))
      (set `self.LockerCurrentState` NewState)
      (if (and (`PrimitiveComponent.IsOverlappingActor` (`self.Box`) (`GameplayStatics.GetPlayerCharacter` 0)) (not (`self.IsActivatedByContact`)))
        (`self.ToggleWidget` true)))))

(fn `ActivateLocker`)

(fn `ToggleWidget`
  (params (Activate :type Boolean))
  (if (`|EnumEquality` (`self.LockerCurrentState`) "NewEnumerator3")
    (bind _ascharacter_bp (cast `/Game/Blueprints/System/Character_BP` (`GameplayStatics.GetPlayerCharacter` 0)))
    (`/Game/UI/InterfaceTest_UW.DisplayInteraction` (`/Game/Blueprints/System/Character_BP.Interface` _ascharacter_bp) Activate)))

(fn `UserConstructionScript`
  (`parent.UserConstructionScript`))