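; Slab-style locker activator that shows its locker state through the material and height of its Cube.
; It extends the parent's ChangeLockerState, then switches on the current state to swap materials.
; Pressed and Valid lower the slab, with a beep only on Pressed, while Unpressed and Deactivated raise it and Invalid changes only the material.
; Construction and BeginPlay both apply the unpressed material.
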(event `self.ReceiveBeginPlay`
  (`parent.ReceiveBeginPlay`)
  (`self.ChangeMaterial` (`self.UnpressedMaterial`)))

(event `self.ChangeLockerState`
  (params (NewState :type "/Game/Enums/CustomLockerState_E Enum" :default "NewEnumerator3"))
  (`parent.ChangeLockerState` NewState)
  (switch `/Game/Enums/CustomLockerState_E` (`self.LockerCurrentState`)
    (:`NewEnumerator3`
      (`self.ChangeMaterial` (`self.UnpressedMaterial`) :!label _label)
      (`SceneComponent.K2_SetRelativeLocation` (`self.Cube`) (0.0 0.0 25.0) false false))
    (:`NewEnumerator2`
      (`self.TryStartSound` "/Game/Sounds/Mechanics/MS_Beep_Simple.MS_Beep_Simple" 0.5 1.0)
      (`self.ChangeMaterial` (`self.PressedMaterial`))
      (`SceneComponent.K2_SetRelativeLocation` (`self.Cube`) (0.0 0.0 15.0) false false :!label _label_2))
    (:`NewEnumerator1`
      (`self.ChangeMaterial` (`self.ValidMaterial`))
      (goto _label_2))
    (:`NewEnumerator0`
      (`self.ChangeMaterial` (`self.InvalidMaterial`)))
    (:`NewEnumerator4`
      (goto _label))))

(fn `ChangeMaterial`
  (params (NewMaterial :type "Material Object Reference"))
  (`PrimitiveComponent.SetMaterial` (`self.Cube`) 0 NewMaterial))

(fn `UserConstructionScript`
  (`parent.UserConstructionScript`)
  (`self.ChangeMaterial` (`self.UnpressedMaterial`)))