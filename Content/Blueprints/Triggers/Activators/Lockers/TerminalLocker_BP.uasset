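; TerminalLocker_BP is a terminal-style locker activator, a child Blueprint that gives visual and audio feedback for its parent's locker state.
; It overrides ChangeLockerState to swap button, screen and padlock plane materials, showing green and unlocked for Pressed or Valid, red and locked otherwise.
; Pressed plays a click sound, and the button sinks for Pressed or Valid, rises for Unpressed or Deactivated, and stays put for Invalid.
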(event `self.ReceiveBeginPlay`
  (`parent.ReceiveBeginPlay`)
  (`self.ChangeMaterial` (`self.UnpressedMaterial`)))

(event `self.ChangeLockerState`
  (params (NewState :type "/Game/Enums/CustomLockerState_E Enum" :default "NewEnumerator3"))
  (`parent.ChangeLockerState` NewState)
  (switch `/Game/Enums/CustomLockerState_E` (`self.LockerCurrentState`)
    (:`NewEnumerator3`
      (`self.ChangeMaterial` (`self.UnpressedMaterial`) :!label _label)
      (`PrimitiveComponent.SetMaterial` (`self.Screen`) 0 "/Game/Materials/BasicColors/M_OldRed.M_OldRed")
      (`PrimitiveComponent.SetMaterial` (`self.Plane`) 0 "/Game/Materials/LockPadlock_M.LockPadlock_M")
      (`SceneComponent.K2_SetRelativeLocation` (`self.Button`) (0.0 0.0 15.0) false false))
    (:`NewEnumerator2`
      (`self.TryStartSound` "/Game/Sounds/Mechanics/SC_RandomClick.SC_RandomClick" 0.7 1.0)
      (`self.ChangeMaterial` (`self.ValidMaterial`) :!label _label_2)
      (`PrimitiveComponent.SetMaterial` (`self.Screen`) 0 "/Game/Materials/BasicColors/M_OldGreen.M_OldGreen")
      (`PrimitiveComponent.SetMaterial` (`self.Plane`) 0 "/Game/Materials/UnlockPadlock_M.UnlockPadlock_M")
      (`SceneComponent.K2_SetRelativeLocation` (`self.Button`) (0.0 0.0 0.0) false false))
    (:`NewEnumerator1`
      (goto _label_2))
    (:`NewEnumerator0`
      (`self.ChangeMaterial` (`self.InvalidMaterial`))
      (`PrimitiveComponent.SetMaterial` (`self.Screen`) 0 "/Game/Materials/BasicColors/M_OldRed.M_OldRed")
      (`PrimitiveComponent.SetMaterial` (`self.Plane`) 0 "/Game/Materials/LockPadlock_M.LockPadlock_M"))
    (:`NewEnumerator4`
      (goto _label))))

(fn `ChangeMaterial`
  (params (NewMaterial :type "Material Object Reference"))
  (`PrimitiveComponent.SetMaterial` (`self.Button`) 0 NewMaterial))

(fn `UserConstructionScript`
  (`parent.UserConstructionScript`)
  (`self.ChangeMaterial` (`self.UnpressedMaterial`)))