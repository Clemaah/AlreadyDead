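; Interactive blue can distributor activator that ejects one physics can per player interaction, with a short cooldown between uses.
; On BeginPlay it caches the meshes under CansContainer, then each interaction pushes the next one out and toggles the player's interaction prompt.
; At the can threshold it locks, Tick raises the door over a timed duration, then it releases every can and gives them another impulse after a delay.
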(event `self.ReceiveBeginPlay`
  (`parent.ReceiveBeginPlay`)
  (for _array_element (`SceneComponent.GetChildrenComponents` (`self.CansContainer`) false)
    (bind _asstatic_mesh_component (cast `StaticMeshComponent` _array_element))
    (`KismetArrayLibrary.Array_Add` (`self.Cans`) _asstatic_mesh_component)))

(event `self.Interact`
  (`parent.Interact`)
  (if (not (`self.IsTemporaryBlocked`))
    (`self.ToggleWidget` false)
    (set `self.IsTemporaryBlocked` true)
    (bind _result (`/Engine/EditorBlueprintResources/StandardMacros.IncrementInt` (`self.CurrentCan`))
      (:`  `
        (`self.GetCan` (`|GetArrayItem` (`self.Cans`) _result))
        (`KismetSystemLibrary.Delay` 0.3)
        (bind _output_get (set `self.IsTemporaryBlocked` (== (`self.CurrentCan`) (`self.CansThreshold`))))
        (if _output_get
          (set `self.OpenTimer` (`self.OpenDuration`))
          (elif (`PrimitiveComponent.IsOverlappingActor` (`self.Box`) (`GameplayStatics.GetPlayerCharacter` 0))
            (`self.ToggleWidget` true)))))))

(event `self.ReceiveTick`
  (params (DeltaSeconds :type "Float (single-precision)"))
  (bind _returnvalue (`GameplayStatics.GetWorldDeltaSeconds`))
  (`parent.ReceiveTick` DeltaSeconds)
  (if (> (`self.OpenTimer`) 0.0)
    (set `self.OpenTimer` (- (`self.OpenTimer`) _returnvalue))
    (`SceneComponent.K2_AddWorldOffset` (`self.Door`) (`KismetMathLibrary.MakeVector` 0.0 0.0 (/ (* _returnvalue 20.0) (`self.OpenDuration`))) false false)
    (if (<= (`self.OpenTimer`) 0.0)
      (for _array_element (`self.Cans`)
        (`self.GetCan` _array_element))
      (`KismetSystemLibrary.Delay` 3.0)
      (for _array_element_2 (`self.Cans`)
        (`PrimitiveComponent.AddImpulse` _array_element_2 (* (`self.GetActorRightVector`) 1000.0) "None" false)))))

(fn `GetCan`
  (params (Can :type "StaticMeshComponent Object Reference"))
  (`PrimitiveComponent.SetSimulatePhysics` Can true)
  (`PrimitiveComponent.AddImpulse` Can (* (`self.GetActorRightVector`) 150.0) "None" true))

(fn `ToggleWidget`
  (params (Activate :type Boolean))
  (if (not (`self.IsTemporaryBlocked`))
    (bind _ascharacter_bp (cast `/Game/Blueprints/System/Character_BP` (`GameplayStatics.GetPlayerCharacter` 0)))
    (`/Game/UI/InterfaceTest_UW.DisplayInteraction` (`/Game/Blueprints/System/Character_BP.Interface` _ascharacter_bp) Activate)))

(fn `UserConstructionScript`)