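; Generator lever activator that the player can interact with to trigger linked activables.
; Interacting plays a lever sound and blocks further interaction while Tick rolls the Moveable component between beginning and ending angles.
; A float curve sampled by elapsed time drives the rotation, without a Timeline node.
; When the block delay elapses, it unblocks and calls the trigger delegate, so activation follows the lever motion.
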(event `self.ReceiveBeginPlay`
  (`parent.ReceiveBeginPlay`)
  (`SceneComponent.K2_SetRelativeRotation` (`self.Moveable`) (`KismetMathLibrary.MakeRotator` (`self.BeginningAngle`)) false false))

(event `self.Interact`
  (`parent.Interact`)
  (if (not (`self.IsTemporaryBlocked`))
    (set `self.IsTemporaryBlocked` true)
    (set `self.TimerBlock` 0.0)
    (`self.TryStartSound` "/Game/Sounds/Mechanics/MS_Lever.MS_Lever" 1.0 1.0)))

(event `self.ReceiveTick`
  (params (DeltaSeconds :type "Float (single-precision)"))
  (`parent.ReceiveTick` DeltaSeconds)
  (if (`self.IsTemporaryBlocked`)
    (bind _output_get (set `self.TimerBlock` (+ DeltaSeconds (`self.TimerBlock`))))
    (`self.UpdateRotation` (`CurveFloat.GetFloatValue` (`self.AlphaRotation`) _output_get))
    (if (>= _output_get (`self.BlockDelay`))
      (set `self.IsTemporaryBlocked` false)
      (`self.TriggerActivablesDelegate`))))

(fn `UpdateRotation`
  (params (TimelineValue :type "Float (double-precision)"))
  (`SceneComponent.K2_SetRelativeRotation` (`self.Moveable`) (`KismetMathLibrary.RLerp` (`KismetMathLibrary.MakeRotator` (`self.BeginningAngle`)) (`KismetMathLibrary.MakeRotator` (`self.EndingAngle`)) TimelineValue true) false false))

(fn `UserConstructionScript`
  (`parent.UserConstructionScript`))