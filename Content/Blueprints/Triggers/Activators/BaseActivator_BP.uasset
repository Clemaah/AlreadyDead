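; Base activator trigger that lets the player interact by key press while in range, meant for child Blueprints to override Interact.
; Range events inherited from the parent bind and unbind the character's InteractionKeyPressed dispatcher and optionally toggle the interaction prompt.
; For unique use, Interact clears the box overlap bindings, hides the prompt and unbinds all listeners from the key event.
; Overrides of Interact are expected to call TriggerActivablesDelegate, which this base graph does not call.
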(event `self.PlayerInRange`
  (params (OverlappedComponent :type "PrimitiveComponent Object Reference") (OtherActor :type "Actor Object Reference") (OtherComp :type "PrimitiveComponent Object Reference") (OtherBodyIndex :type Integer) (bFromSweep :type Boolean) (SweepResult :type "HitResult Structure (by ref)"))
  ;[1 1 1] Bind/unbind when in range with the interaction button pressed event
  (bind _ascharacter_bp (cast `/Game/Blueprints/System/Character_BP` OtherActor))
  (add `/Game/Blueprints/System/Character_BP.InteractionKeyPressed` _ascharacter_bp (`|CreateDelegate` :!event `Interact`))
  (if (`self.DisplayWidget`)
    (`self.ToggleWidget` true)))

(event `self.PlayerOutOfRange`
  (params (OverlappedComponent :type "PrimitiveComponent Object Reference") (OtherActor :type "Actor Object Reference") (OtherComp :type "PrimitiveComponent Object Reference") (OtherBodyIndex :type Integer))
  ;[1 1 1] Bind/unbind when in range with the interaction button pressed event
  (bind _ascharacter_bp (cast `/Game/Blueprints/System/Character_BP` OtherActor))
  (remove `/Game/Blueprints/System/Character_BP.InteractionKeyPressed` _ascharacter_bp (`|CreateDelegate` :!event `Interact`))
  (if (`self.DisplayWidget`)
    (`self.ToggleWidget` false)))

(event `Interact`
  ;[1 1 1] Unbind all events when it's for unique use
  (if (`self.IsForUniqueUse`)
    (clear `PrimitiveComponent.OnComponentBeginOverlap` (`self.Box`))
    (clear `PrimitiveComponent.OnComponentEndOverlap` (`self.Box`))
    (bind _ascharacter_bp (cast `/Game/Blueprints/System/Character_BP` (`GameplayStatics.GetPlayerCharacter` 0)))
    (`/Game/UI/InterfaceTest_UW.DisplayInteraction` (`/Game/Blueprints/System/Character_BP.Interface` _ascharacter_bp) false)
    (clear `/Game/Blueprints/System/Character_BP.InteractionKeyPressed` _ascharacter_bp)))

(fn `ToggleWidget`
  (params (Activate :type Boolean))
  (bind _ascharacter_bp (cast `/Game/Blueprints/System/Character_BP` (`GameplayStatics.GetPlayerCharacter` 0)))
  (`/Game/UI/InterfaceTest_UW.DisplayInteraction` (`/Game/Blueprints/System/Character_BP.Interface` _ascharacter_bp) Activate))

(fn `UserConstructionScript`)