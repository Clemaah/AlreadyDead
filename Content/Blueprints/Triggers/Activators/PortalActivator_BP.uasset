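; Portal activator that the player powers with five soul collectables and then uses to teleport.
; Entering the sphere reads the character's souls, and Tick switches on child-actor receptacles one by one on a timer; leaving before activation resets them.
; With all five displayed, interacting removes the souls, fires parent activation and portal effects, disables the sphere and starts teleportation.
; Once activated, further interactions only start a shorter teleportation.
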(event `self.ReceiveBeginPlay`
  (`parent.ReceiveBeginPlay`)
  (for _array_element (`SceneComponent.GetChildrenComponents` (`self.ReceptaclesContainer`) false)
    (bind _aschild_actor_component (cast `ChildActorComponent` _array_element))
    (bind _asreceptacle_bp (cast `/Game/Blueprints/Receptacle_BP` (`ChildActorComponent.ChildActor` _aschild_actor_component)))
    (`KismetArrayLibrary.Array_Add` (`self.Receptacles`) _asreceptacle_bp)))

(event `self.Sphere.OnComponentBeginOverlap`
  (params (OverlappedComponent :type "PrimitiveComponent Object Reference") (OtherActor :type "Actor Object Reference") (OtherComp :type "PrimitiveComponent Object Reference") (OtherBodyIndex :type Integer) (bFromSweep :type Boolean) (SweepResult :type "HitResult Structure (by ref)"))
  (bind _ascharacter_bp (cast `/Game/Blueprints/System/Character_BP` OtherActor))
  (set `self.AvailableSouls` (`KismetMathLibrary.Min` (`/Game/Blueprints/System/Character_BP.GetCollectable` _ascharacter_bp "/Game/Blueprints/Collectables/SoulCollectable_BP.SoulCollectable_BP_C") 5))
  (set `self.ApparitionTimer` (`self.ApparitionDelay`)))

(event `self.Sphere.OnComponentEndOverlap`
  (params (OverlappedComponent :type "PrimitiveComponent Object Reference") (OtherActor :type "Actor Object Reference") (OtherComp :type "PrimitiveComponent Object Reference") (OtherBodyIndex :type Integer))
  (cast `/Game/Blueprints/System/Character_BP` OtherActor)
  (if (not (`self.IsActivated`))
    (for _index (range 1 (+ (`self.DisplayedSouls`) 1))
      (`/Game/Blueprints/Receptacle_BP.SwitchActivation` (`|GetArrayItem` (`self.Receptacles`) (- _index 1))))
    (set `self.DisplayedSouls` 0)
    (set `self.AvailableSouls` 0)))

(event `self.Interact`
  (if (`self.IsActivated`)
    (bind _ascharacter_bp (cast `/Game/Blueprints/System/Character_BP` (`GameplayStatics.GetPlayerCharacter` 0)))
    (`/Game/Blueprints/System/Character_BP.StartTeleportation` _ascharacter_bp 0.5)
    (elif (== (`self.DisplayedSouls`) 5)
      (`parent.Interact`)
      (set `self.IsActivated` true)
      (bind _ascharacter_bp_2 (cast `/Game/Blueprints/System/Character_BP` (`GameplayStatics.GetPlayerCharacter` 0)))
      (`/Game/Blueprints/System/Character_BP.RemoveCollectable` _ascharacter_bp_2 "/Game/Blueprints/Collectables/SoulCollectable_BP.SoulCollectable_BP_C" 5)
      (`self.FeedbackActivation`)
      (`PrimitiveComponent.SetCollisionEnabled` (`self.Sphere`) "NoCollision")
      (bind _ascharacter_bp_3 (cast `/Game/Blueprints/System/Character_BP` (`GameplayStatics.GetPlayerCharacter` 0)))
      (`/Game/Blueprints/System/Character_BP.StartTeleportation` _ascharacter_bp_3 1.0))))

(event `self.ReceiveTick`
  (params (DeltaSeconds :type "Float (single-precision)"))
  (`parent.ReceiveTick` DeltaSeconds)
  (if (and (> (`self.AvailableSouls`) 0) (< (`self.DisplayedSouls`) (`self.AvailableSouls`)))
    (bind _output_get (set `self.ApparitionTimer` (- (`self.ApparitionTimer`) (`GameplayStatics.GetWorldDeltaSeconds`))))
    (if (<= _output_get 0.0)
      (`/Game/Blueprints/Receptacle_BP.SwitchActivation` (`|GetArrayItem` (`self.Receptacles`) (`self.DisplayedSouls`)))
      (set `self.ApparitionTimer` (`self.ApparitionDelay`))
      (bind _result (`/Engine/EditorBlueprintResources/StandardMacros.IncrementInt` (`self.DisplayedSouls`))
        (:`  `
          (if (and (== _result 5) (`PrimitiveComponent.IsOverlappingActor` (`self.Box`) (`GameplayStatics.GetPlayerCharacter` 0)))
            (`self.ToggleWidget` true)))))))

(fn `FeedbackActivation`
  (`PrimitiveComponent.SetMaterial` (`self.EmissiveCylinder`) 0 "/Game/Materials/EmissivePurple_M.EmissivePurple_M")
  (`ActorComponent.Activate` (`self.PortalParticles`) false))

(fn `IsOn`
  (returns (IsOn :type Boolean))
  (return (`self.IsFreezedByWord`)))

(fn `ToggleWidget`
  (params (Activate :type Boolean))
  (if (or (`self.IsActivated`) (== (`self.DisplayedSouls`) 5))
    (bind _ascharacter_bp (cast `/Game/Blueprints/System/Character_BP` (`GameplayStatics.GetPlayerCharacter` 0)))
    (`/Game/UI/InterfaceTest_UW.DisplayInteraction` (`/Game/Blueprints/System/Character_BP.Interface` _ascharacter_bp) Activate)))

(fn `UserConstructionScript`)