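; ButtonActivator_BP is a trigger activator button that the player interacts with to fire the TriggerActivables delegate.
; Interact hides the character's interaction prompt, plays a click, pushes the button mesh in, turns it blue and starts a temporary block.
; Tick counts the block delay, then, unless the button is single-use, resets it to red and restores the prompt if the player still overlaps its box.
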(event `self.Interact`
  (`parent.Interact`)
  (if (not (`self.IsTemporaryBlocked`))
    (`self.ToggleWidget` false)
    (set `self.IsTemporaryBlocked` true)
    (set `self.TimerBlock` 0.0)
    (`self.TryStartSound` "/Game/Sounds/Mechanics/SC_RandomClick.SC_RandomClick" 0.8 1.0)
    (`self.TriggerActivablesDelegate`)
    (`SceneComponent.K2_AddRelativeLocation` (`self.Button`) (0.0 -8.0 0.0) false false)
    (`PrimitiveComponent.SetMaterial` (`self.Button`) 0 "/Game/Materials/M_BlueEmissiveButton.M_BlueEmissiveButton")))

(event `self.ReceiveTick`
  (params (DeltaSeconds :type "Float (single-precision)"))
  (`parent.ReceiveTick` DeltaSeconds)
  (if (`self.IsTemporaryBlocked`)
    (bind _output_get (set `self.TimerBlock` (+ DeltaSeconds (`self.TimerBlock`))))
    (if (>= _output_get (`self.BlockDelay`))
      (set `self.IsTemporaryBlocked` false)
      (if (not (`self.IsForUniqueUse`))
        (`SceneComponent.K2_AddRelativeLocation` (`self.Button`) (0.0 8.0 0.0) false false)
        (`PrimitiveComponent.SetMaterial` (`self.Button`) 0 "/Game/Materials/M_RedEmissiveButton.M_RedEmissiveButton")
        (if (`PrimitiveComponent.IsOverlappingActor` (`self.Box`) (`GameplayStatics.GetPlayerCharacter` 0))
          (`self.ToggleWidget` true))))))

(fn `ToggleWidget`
  (params (Activate :type Boolean))
  (if (not (`self.IsTemporaryBlocked`))
    (bind _ascharacter_bp (cast `/Game/Blueprints/System/Character_BP` (`GameplayStatics.GetPlayerCharacter` 0)))
    (`/Game/UI/InterfaceTest_UW.DisplayInteraction` (`/Game/Blueprints/System/Character_BP.Interface` _ascharacter_bp) Activate)))

(fn `UserConstructionScript`
  (`parent.UserConstructionScript`))