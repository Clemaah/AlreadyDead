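; Base trigger Blueprint with a box volume that detects the player and follows the Living or Death World state.
; On BeginPlay it binds the box's begin and end overlaps to empty PlayerInRange and PlayerOutOfRange events, meant for child classes to override.
; It extends the parent's SwitchBehaviour to toggle box collision between query-only and none according to IsOn.
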(event `self.ReceiveBeginPlay`
  (`parent.ReceiveBeginPlay`)
  ;[1 1 1] Call custom event when the player enter/exit the box collider
  (add `PrimitiveComponent.OnComponentBeginOverlap` (`self.Box`) (delegate `PlayerInRange`))
  (add `PrimitiveComponent.OnComponentEndOverlap` (`self.Box`) (delegate `PlayerOutOfRange`)))

(event `PlayerInRange`
  (params (OverlappedComponent :type "PrimitiveComponent Object Reference") (OtherActor :type "Actor Object Reference") (OtherComp :type "PrimitiveComponent Object Reference") (OtherBodyIndex :type Integer) (bFromSweep :type Boolean) (SweepResult :type "HitResult Structure (by ref)"))
  ;[1 1 1] Call custom event when the player enter/exit the box collider
)

(event `PlayerOutOfRange`
  (params (OverlappedComponent :type "PrimitiveComponent Object Reference") (OtherActor :type "Actor Object Reference") (OtherComp :type "PrimitiveComponent Object Reference") (OtherBodyIndex :type Integer))
  ;[1 1 1] Call custom event when the player enter/exit the box collider
)

(event `self.SwitchBehaviour`
  ;[1 1 1] Activate/Deactivate Collision based on current Player location (Living or Death World)
  (`parent.SwitchBehaviour`)
  (`PrimitiveComponent.SetCollisionEnabled` (`self.Box`) (select `bool` (`self.IsOn`) :`false` "NoCollision" :`true` "QueryOnly" :!type "ECollisionEnabled Enum")))

(fn `UserConstructionScript`)