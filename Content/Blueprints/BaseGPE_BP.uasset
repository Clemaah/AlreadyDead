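; Base Blueprint for gameplay elements (GPE) that freeze while the player is in the Death World and resume in the Living World.
; It binds to the player character's world-teleport events, then calls an overridable SwitchBehaviour that toggles actor tick and sound.
; A Tick-driven sound state machine handles delayed starts and tracks playback time, so paused sounds restart where they stopped.
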(event `self.ReceiveBeginPlay`
  (`parent.ReceiveBeginPlay`)
  ;[1 1 1] Variable Initialization
  (`AudioComponent.SetSound` (`self.Audio`) null)
  (bind _ascharacter_bp (cast `/Game/Blueprints/System/Character_BP` (`GameplayStatics.GetPlayerCharacter` 0)))
  (set `self.IsFreezedByWord` (not (`/Game/Blueprints/System/Character_BP.IsInLivingWorld` _ascharacter_bp)))
  (`self.SwitchBehaviour`)
  ;[1 1 1] Binding events to the player's teleportation events
  (add `/Game/Blueprints/System/Character_BP.TpDeathWorld` _ascharacter_bp (`|CreateDelegate` :!event `InDeathWorld`))
  (add `/Game/Blueprints/System/Character_BP.TpLivingWorld` _ascharacter_bp (`|CreateDelegate` :!event `InLivingWorld`)))

(event `InDeathWorld`
  ;[1 1 1] Freezing In Death World
  (set `self.IsFreezedByWord` true)
  (`self.SwitchBehaviour`))

(event `InLivingWorld`
  ;[1 1 1] Unfreezing in Living World
  (set `self.IsFreezedByWord` false)
  (`self.SwitchBehaviour`))

(event `SwitchBehaviour`
  (bind _ison (`self.IsOn`))
  ;[1 1 1] Behaviour switch
  (`self.ChangeSoundState` _ison)
  (`self.SetActorTickEnabled` _ison))

(event `ChangeSoundState`
  (params (Activate :type Boolean))
  ;[1 1 1] Try changing the sound state
  (if Activate
    (`self.TryUnpauseSound`)
    (else
      (`self.TryPauseSound`))))

(event `TryUnpauseSound`
  ;[1 1 1] Trying to unpause the sound. Unpause only if a valid sound is enter and if it is in paused state.
  (`/Engine/EditorBlueprintResources/StandardMacros.IsValid` (`AudioComponent.Sound` (`self.Audio`))
    (:`Is Valid`
      (if (`|EnumEquality` (`self.SoundCurrentState`) "NewEnumerator1")
        (`self.StartSound`)))))

(event `TryPauseSound`
  ;[1 1 1] Trying to pause the sound. Pause only if a valid sound is enter and if it's currently playing.
  (`/Engine/EditorBlueprintResources/StandardMacros.IsValid` (`AudioComponent.Sound` (`self.Audio`))
    (:`Is Valid`
      (if (`|EnumEquality` (`self.SoundCurrentState`) "NewEnumerator2")
        (set `self.SoundCurrentState` "NewEnumerator1")
        (`AudioComponent.Stop` (`self.Audio`))))))

(event `TryStartSound`
  (params (Sound :type "SoundBase Object Reference") (Volume :type "Float (double-precision)") (Pitch :type "Float (double-precision)") (IsUISound :type Boolean))
  ;[1 1 1] Trying to start the sound. Start only if a valid sound.
  (`/Engine/EditorBlueprintResources/StandardMacros.IsValid` Sound
    (:`Is Valid`
      (`AudioComponent.SetSound` (`self.Audio`) Sound)
      (`AudioComponent.SetVolumeMultiplier` (`self.Audio`) Volume)
      (`AudioComponent.SetPitchMultiplier` (`self.Audio`) Pitch)
      (`AudioComponent.SetUISound` (`self.Audio`) IsUISound)
      (set `self.TimerSoundDelay` 0.0)
      (set `self.SoundCurrentState` "NewEnumerator3"))))

(event `self.ReceiveTick`
  (params (DeltaSeconds :type "Float (single-precision)"))
  ;[1 1 1] Tick event
  (switch `/Game/Enums/CustomSoundState_E` (`self.SoundCurrentState`)
    (:`NewEnumerator3`
      (bind _output_get (set `self.TimerSoundDelay` (+ DeltaSeconds (`self.TimerSoundDelay`))))
      (if (>= _output_get (`self.SoundDelay`))
        (set `self.TimerPlaying` 0.0)
        (`self.StartSound`)))
    (:`NewEnumerator2`
      (if (`AudioComponent.IsPlaying` (`self.Audio`))
        (set `self.TimerPlaying` (+ DeltaSeconds (`self.TimerPlaying`)))
        (else
          (set `self.SoundCurrentState` "NewEnumerator0"))))))

(fn `IsOn`
  (returns (IsOn :type Boolean))
  (return (not (`self.IsFreezedByWord`))))

(fn `StartSound`
  (`AudioComponent.Play` (`self.Audio`) (`self.TimerPlaying`))
  (set `self.SoundCurrentState` "NewEnumerator2"))

(fn `UserConstructionScript`)