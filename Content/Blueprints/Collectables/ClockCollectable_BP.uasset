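; Clock collectable that animates its Montre watch component and plays a quiet 2D pickup sound when collected.
; Each Tick spins the watch on yaw and sets its relative Z from GetNewLocation.
; GetNewLocation contains a time-based sine bob using movement speed and amplitude, though that expression appears unconnected to the function's output.
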(event `self.ReceiveTick`
  (params (DeltaSeconds :type "Float (single-precision)"))
  (`SceneComponent.K2_SetRelativeLocation` (`self.Montre`) (`KismetMathLibrary.MakeVector` 0.0 0.0 (* (`KismetMathLibrary.Sin` (* (`GameplayStatics.GetTimeSeconds`) (`self.MovementSpeed`))) (`self.MovementAmplitude`))) false false)
  (`SceneComponent.K2_AddRelativeRotation` (`self.Montre`) (`KismetMathLibrary.MakeRotator` 0.0 0.0 (`self.RotationSpeed`)) false false))

(event `self.On Collect`
  (`GameplayStatics.PlaySound2D` "/Game/Sounds/Mechanics/MS_Collectible.MS_Collectible" 0.3 1.0 0.0 null null))

(fn `UserConstructionScript`
  (`parent.UserConstructionScript`))