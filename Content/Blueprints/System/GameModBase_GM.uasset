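; Base game mode that sets up the sky and background music, and switches time of day as the player teleports between the death and living worlds.
; On BeginPlay it spawns a GoodSky actor, applies cloud, effect and star settings, and starts at the death world hour.
; It binds to the player character's teleport dispatchers, so each teleport sets that world's hour and triggers a realtime sky update.
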(event `self.ReceiveBeginPlay`
  (bind _sky (`self.Sky`))
  (bind _returnvalue (`|SpawnActorFromClass` "/Game/GoodSky/Blueprint/BP_GoodSky.BP_GoodSky_C" (`self.GetLevelTransform`) "Undefined" "MultiplyWithRoot" null null))
  (set `self.Sky` _returnvalue)
  (set `/Game/GoodSky/Blueprint/BP_GoodSky.SkyCloudsStyle` "NewEnumerator1" _sky)
  (set `/Game/GoodSky/Blueprint/BP_GoodSky.SkyCloudsCoveragePreset` "NewEnumerator4" _sky)
  (set `/Game/GoodSky/Blueprint/BP_GoodSky.SkyEffect` "NewEnumerator5" _sky)
  (set `/Game/GoodSky/Blueprint/BP_GoodSky.SkyMesh` "NewEnumerator1" _sky)
  (set `/Game/GoodSky/Blueprint/BP_GoodSky.Sun Direction` "NewEnumerator1" _sky)
  (set `/Game/GoodSky/Blueprint/BP_GoodSky.Stars Brightness` 0.2 _sky)
  (`self.ChangingHour` (`self.DeathWorldHour`))
  (`GameplayStatics.PlaySound2D` "/Game/Sounds/Music/MS_BackgroundMusic.MS_BackgroundMusic" 0.1 1.0 0.0 null null) ; Playing the background music.
  ;[1 1 1] Changing the sky when player teleportation occurs
  (bind _ascharacter_bp (cast `/Game/Blueprints/System/Character_BP` (`GameplayStatics.GetPlayerCharacter` 0)))
  (add `/Game/Blueprints/System/Character_BP.TpDeathWorld` _ascharacter_bp (delegate `DeathHour`))
  (add `/Game/Blueprints/System/Character_BP.TpLivingWorld` _ascharacter_bp (delegate `LivingHour`)))

(event `DeathHour`
  ;[1 1 1] Changing the sky when player teleportation occurs
  (`self.ChangingHour` (`self.DeathWorldHour`)))

(event `LivingHour`
  ;[1 1 1] Changing the sky when player teleportation occurs
  (`self.ChangingHour` (`self.LivingWorldHour`)))

(fn `ChangingHour`
  (params (NewHour :type "Float (double-precision)"))
  (set `/Game/GoodSky/Blueprint/BP_GoodSky.└ Time of Day ( For Custom Mode )` NewHour (`self.Sky`))
  (`/Game/GoodSky/Blueprint/BP_GoodSky.GoodSky Realtime Update` (`self.Sky`)))

(fn `UserConstructionScript`
  (`parent.UserConstructionScript`))