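; Player character that switches between a living world and a death world, tracking play time, death count and collectables.
; World switches offset the actor by a fixed spacing; the dead state gets a ghost overlay and faster walk speed.
; Delayed teleportation fades a black screen and ragdolls the living body before switching.
; A map-based inventory feeds clock and soul counts to the HUD, and input triggers interaction, switching and soul granting.
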(event `self.ReceiveBeginPlay`
  (bind _returnvalue (`GameplayStatics.GetPlayerController` 0))
  (`parent.ReceiveBeginPlay`)
  (set `self.WorldsSpacing` (`/Game/Editor/WorldOrigin_BF.GetWorldsSpacing`))
  (bind _returnvalue_2 (`|CreateWidget` "/Game/UI/WB_Interface.WB_Interface_C"))
  (bind _output_get (set `self.Interface` _returnvalue_2))
  (`UserWidget.AddToViewport` _output_get 0)
  (bind _returnvalue_3 (`|CreateWidget` "/Game/UI/WB_BlackScreen.WB_BlackScreen_C"))
  (bind _output_get_2 (set `self.BlackScreen` _returnvalue_3))
  (`UserWidget.AddToViewport` _output_get_2 0)
  (`/Game/UI/WB_BlackScreen.FadeInEvent` _returnvalue_3 "Reverse" 1.0)
  (`self.ChangeSpeed` (not (`self.IsInLivingWorld`)))
  (`GameplayStatics.SetGamePaused` false)
  (set `PlayerController.bShowMouseCursor` false _returnvalue)
  (`WidgetBlueprintLibrary.SetInputMode_GameOnly` _returnvalue))

(event `self.ReceiveTick`
  (params (DeltaSeconds :type "Float (single-precision)"))
  (`parent.ReceiveTick` DeltaSeconds)
  (set `self.Timer` (+ (`self.Timer`) DeltaSeconds)))

(event `EnhancedInput|/Game/ThirdParty/ThirdPerson/Input/Actions/IA_Interact`
  (params (ActionValue :type Boolean) (ElapsedSeconds :type "Float (double-precision)") (TriggeredSeconds :type "Float (double-precision)") (InputAction :type "InputAction Object Reference" :default "/Game/ThirdParty/ThirdPerson/Input/Actions/IA_Interact.IA_Interact"))
  (:`Triggered`
    (`self.InteractionKeyPressed`)))

(event `EnhancedInput|/Game/ThirdParty/ThirdPerson/Input/Actions/IA_SoulGive`
  (params (ActionValue :type Boolean) (ElapsedSeconds :type "Float (double-precision)") (TriggeredSeconds :type "Float (double-precision)") (InputAction :type "InputAction Object Reference" :default "/Game/ThirdParty/ThirdPerson/Input/Actions/IA_SoulGive.IA_SoulGive"))
  (:`Triggered`
    (`self.AddCollectable` "/Game/Blueprints/Collectables/SoulCollectable_BP.SoulCollectable_BP_C" 1)))

(event `EnhancedInput|/Game/ThirdParty/ThirdPerson/Input/Actions/IA_WorldSwich`
  (params (ActionValue :type Boolean) (ElapsedSeconds :type "Float (double-precision)") (TriggeredSeconds :type "Float (double-precision)") (InputAction :type "InputAction Object Reference" :default "/Game/ThirdParty/ThirdPerson/Input/Actions/IA_WorldSwich.IA_WorldSwich"))
  (:`Triggered`
    (`self.WorldSwitch`)))

(event `StartTeleportation`
  (params (Delay :type "Float (double-precision)"))
  (`/Game/UI/WB_BlackScreen.FadeInEvent` (`self.BlackScreen`) "Forward" Delay)
  (if (`self.IsInLivingWorld`)
    (`self.EnableRagdoll`))
  (`KismetSystemLibrary.Delay` (+ Delay 0.5))
  (`self.WorldSwitch`)
  (`/Game/UI/WB_BlackScreen.FadeInEvent` (`self.BlackScreen`) "Reverse" 0.0))

(fn `ActualizeInterface`
  (`/Game/UI/WB_Interface.Actualize` (`self.Interface`) (`self.GetCollectable` "/Game/Blueprints/Collectables/ClockCollectable_BP.ClockCollectable_BP_C") (`self.GetCollectable` "/Game/Blueprints/Collectables/SoulCollectable_BP.SoulCollectable_BP_C")))

(fn `AddCollectable`
  (params (Collectable :type "/Game/Blueprints/Collectables/BaseCollectable_BP Class Reference") (Quantity :type Integer))
  (bind _inventory (`self.Inventory`))
  (`BlueprintMapLibrary.Map_Add` _inventory Collectable (+ (`BlueprintMapLibrary.Map_Find` _inventory Collectable) Quantity))
  (`self.ActualizeInterface`))

(fn `ChangeCharacterMesh`
  (params (IsDead :type Boolean))
  (if IsDead
    (`MeshComponent.SetOverlayMaterial` (`self.Mesh`) "/Game/Materials/VFXMaterials/M_Ghost_Overlay.M_Ghost_Overlay")
    (else
      (`MeshComponent.SetOverlayMaterial` (`self.Mesh`) null))))

(fn `ChangeSpeed`
  (params (IsDead :type Boolean))
  (bind _returnvalue (`KismetMathLibrary.Abs` (`self.DeathVariationSpeed`)))
  (bind _output_get (set `self.DeathVariationSpeed` (`KismetMathLibrary.SelectFloat` _returnvalue (* _returnvalue -1.0) IsDead)))
  (set `CharacterMovementComponent.MaxWalkSpeed` (+ _output_get (`self.WalkSpeed`)) (`self.CharacterMovement`)))

(fn `ContainCollectable`
  (params (Collectable :type "/Game/Blueprints/Collectables/BaseCollectable_BP Class Reference"))
  (returns (IsContained :type Boolean))
  (return (`BlueprintMapLibrary.Map_Contains` (`self.Inventory`) Collectable)))

(fn `DisableRagdoll`
  (`PrimitiveComponent.SetSimulatePhysics` (`self.Mesh`) false)
  (`PrimitiveComponent.SetCollisionProfileName` (`self.Mesh`) "CharacterMesh" true)
  (`CharacterMovementComponent.SetMovementMode` (`self.CharacterMovement`) "MOVE_Walking" 0)
  (`PrimitiveComponent.SetCollisionEnabled` (`self.CapsuleComponent`) "QueryAndPhysics")
  (`SceneComponent.K2_AttachToComponent` (`self.Mesh`) (`self.CapsuleComponent`) "None" "SnapToTarget" "KeepRelative" "KeepRelative" true)
  (`SceneComponent.K2_SetRelativeLocationAndRotation` (`self.Mesh`) (0.0 0.0 -89.0) (struct :`Yaw` 270.0) false false))

(fn `EnableRagdoll`
  (`CharacterMovementComponent.DisableMovement` (`self.CharacterMovement`))
  (`PrimitiveComponent.SetCollisionEnabled` (`self.CapsuleComponent`) "NoCollision")
  (`PrimitiveComponent.SetCollisionProfileName` (`self.Mesh`) "Ragdoll" true)
  (`PrimitiveComponent.SetSimulatePhysics` (`self.Mesh`) true))

(fn `GetCollectable`
  (params (Collectable :type "/Game/Blueprints/Collectables/BaseCollectable_BP Class Reference"))
  (returns (Quantity :type Integer))
  (return (`BlueprintMapLibrary.Map_Find` (`self.Inventory`) Collectable)))

(fn `RemoveCollectable`
  (params (Collectable :type "/Game/Blueprints/Collectables/BaseCollectable_BP Class Reference") (Quantity :type Integer))
  (returns (IsRemoved :type Boolean))
  (if (>= (`self.GetCollectable` Collectable) Quantity)
    (bind _result (`/Engine/EditorBlueprintResources/StandardMacros.NegateInt` Quantity)
      (:`  `
        (`self.AddCollectable` Collectable _result)
        (`self.ActualizeInterface`)
        (return true)))
    (else
      (return false))))

(fn `ToDeathWorld`
  (`self.TpDeathWorld`)
  (if (not (`|EnumEquality` (`CharacterMovementComponent.MovementMode` (`self.CharacterMovement`)) "MOVE_Flying"))
    (`self.DisableRagdoll`))
  (`self.K2_AddActorWorldOffset` (`KismetMathLibrary.NegateVector` (`self.WorldsSpacing`)) false true)
  (`self.ChangeCharacterMesh` true)
  (`self.ChangeSpeed` true)
  (`/Engine/EditorBlueprintResources/StandardMacros.IncrementInt` (`self.DeathCount`)))

(fn `ToLivingWorld`
  (`self.K2_AddActorWorldOffset` (`self.WorldsSpacing`) false true)
  (`self.ChangeCharacterMesh` false)
  (`self.ChangeSpeed` false)
  (`self.TpLivingWorld`))

(fn `UserConstructionScript`
  (`parent.UserConstructionScript`))

(fn `WorldSwitch`
  (bind _output_get (set `self.IsInLivingWorld` (not (`self.IsInLivingWorld`))))
  (if _output_get
    (`self.ToLivingWorld`)
    (else
      (`self.ToDeathWorld`))))