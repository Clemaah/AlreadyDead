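; Blueprint function library for WorldOrigin_BP actors, which mark the origins of the Living World and Death World.
; The validity check counts placed origins per world and returns true only when each has exactly one, printing a red on-screen error for missing or duplicate ones.
; The location lookup returns the first matching origin's position, or prints an error and returns a zero vector.
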(fn `CheckWorldsOriginValidity`
  (returns (AreValid :type Boolean))
  (locals (LivingWorldNumber :type Integer) (DeathWorldNumber :type Integer))
  (bind _livingworldnumber (`local.LivingWorldNumber`))
  (bind _deathworldnumber (`local.DeathWorldNumber`))
  (bind _returnvalue (== 1 _deathworldnumber))
  (bind _returnvalue_2 (== 1 _livingworldnumber))
  (bind _outactors (`GameplayStatics.GetAllActorsOfClass` null "/Game/Blueprint/WorldOrigin/WorldOrigin_BP.WorldOrigin_BP_C"))
  (for _array_element _outactors
    (switch `/Game/Blueprint/WorldOrigin/WorldsEnum` (`/Game/Blueprint/WorldOrigin/WorldOrigin_BP.World` _array_element)
      (:`NewEnumerator0`
        (`/Engine/EditorBlueprintResources/StandardMacros.IncrementInt` (`local.LivingWorldNumber`)))
      (:`NewEnumerator1`
        (`/Engine/EditorBlueprintResources/StandardMacros.IncrementInt` (`local.DeathWorldNumber`)))))
  (`|ExecutionSequence`
    (:`then_0`
      (if (not _returnvalue_2)
        (`self.PrintWorldOriginError` "NewEnumerator0" _livingworldnumber)))
    (:`then_1`
      (if (not _returnvalue)
        (`self.PrintWorldOriginError` "NewEnumerator1" _deathworldnumber)))
    (:`then_2`
      (return (and _returnvalue_2 _returnvalue)))))

(fn `GetWorldOriginLocation`
  (params (World :type "/Game/Blueprint/WorldOrigin/WorldsEnum Enum" :default "NewEnumerator0"))
  (returns (Location :type "Vector Structure"))
  (bind _outactors (`GameplayStatics.GetAllActorsOfClass` null "/Game/Blueprint/WorldOrigin/WorldOrigin_BP.WorldOrigin_BP_C"))
  (for _array_element _outactors
    (if (`|EnumEquality` (`/Game/Blueprint/WorldOrigin/WorldOrigin_BP.World` _array_element) World)
      (return (`Actor.K2_GetActorLocation` _array_element))))
  (`KismetSystemLibrary.PrintString` null "error: No world's origin found." true true (struct :`R` 1.0 :`A` 1.0) 10.0)
  (return (0.0 0.0 0.0)))

(fn `PrintWorldOriginError`
  (params (World :type "/Game/Blueprint/WorldOrigin/WorldsEnum Enum" :default "NewEnumerator0") (NumberOfWorldOrigin :type Integer))
  (locals (ErrorMessage :type String) (WorldName :type String))
  (set `local.WorldName` (`|GetEnumeratorNameAsString` World))
  (if (== NumberOfWorldOrigin 0)
    (set `local.ErrorMessage` (`KismetStringLibrary.Concat_StrStr` "error: No " (`local.WorldName`) "'s Origin were found."))
    (else
      (set `local.ErrorMessage` (`KismetStringLibrary.Concat_StrStr` "error: There is " (`KismetStringLibrary.Conv_IntToString` NumberOfWorldOrigin) " occurences of " (`local.WorldName`) "'s Origin. There can be only one at a time."))))
  (`KismetSystemLibrary.PrintString` null (`local.ErrorMessage`) true true (struct :`R` 1.0 :`A` 1.0) 10.0))