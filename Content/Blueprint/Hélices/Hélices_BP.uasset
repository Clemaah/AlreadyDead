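; Hélices_BP is a propeller actor that spins and has collision only while the player is in the living world.
; Each Tick rotates it locally on pitch by Speed scaled by delta time, then polls IsInLivingsWorld on the player's Character_BP.
; That flag switches Speed between spinning and stopped and toggles the Box component's collision between query-and-physics and none.
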(event `self.ReceiveTick`
  (params (DeltaSeconds :type "Float (single-precision)"))
  (bind (_returnvalue_roll _returnvalue_pitch) (`KismetMathLibrary.BreakRotator` (`KismetMathLibrary.MakeRotator` 0.0 (`self.speed`))))
  ;[1 1 1] Rotation
  (`self.K2_AddActorLocalRotation` (`KismetMathLibrary.MakeRotator` 0.0 (* _returnvalue_pitch DeltaSeconds)))
  ;[1 1 1] Check if the player is on the livingworld or not
  (bind _ascharacter_bp (cast `/Game/Blueprint/Character_BP` (`GameplayStatics.GetPlayerCharacter` 0)))
  (if (`/Game/Blueprint/Character_BP.IsInLivingsWorld` _ascharacter_bp)
    ;[1 1 1] Adapt rotation and collision
    (set `self.speed` 180.0)
    (`PrimitiveComponent.SetCollisionEnabled` (`self.Box`) "QueryAndPhysics")
    (else
      (set `self.speed` 0.0)
      (`PrimitiveComponent.SetCollisionEnabled` (`self.Box`) "NoCollision"))))

(fn `UserConstructionScript`)