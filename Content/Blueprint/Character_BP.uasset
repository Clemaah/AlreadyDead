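; Player character Blueprint that switches between a living and a death world and carries collectables such as coins and souls.
; WorldSwich toggles the state, offsets the actor by WorldsSpacing, applies or clears a ghost overlay material and calls the matching world event.
; An inventory map keyed by collectable class backs add, remove and query functions.
; Input forwards interaction and grants debug souls, while Tick prints counts and control hints.
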(event `self.ReceiveBeginPlay`
  (`parent.ReceiveBeginPlay`)
  (set `self.WorldsSpacing` (`/Game/Blueprint/WorldOrigin/WorldsOriginFunctions.GetWorldsSpacing`))
  (bind _returnvalue (`|CreateWidget` "/Game/UI/InterfaceTest_UW.InterfaceTest_UW_C"))
  (`UserWidget.AddToViewport` _returnvalue 0))

(event `self.ReceiveTick`
  (params (DeltaSeconds :type "Float (single-precision)"))
  (`parent.ReceiveTick` DeltaSeconds)
  ;[1 1 1] Debug Print
  (`KismetSystemLibrary.PrintString` (`KismetStringLibrary.Concat_StrStr` (`KismetStringLibrary.Conv_IntToString` (`self.GetCollectable` "/Game/Blueprint/Collectable/CoinCollectable_BP.CoinCollectable_BP_C")) " Pièces") true false (struct :`R` 0.880208 :`G` 0.554437 :`B` 0.022922 :`A` 1.0) 0.0)
  (`KismetSystemLibrary.PrintString` (`KismetStringLibrary.Concat_StrStr` (`KismetStringLibrary.Conv_IntToString` (`self.GetCollectable` "/Game/Blueprint/Collectable/SoulCollectable_BP.SoulCollectable_BP_C")) " Âmes") true false (struct :`R` 0.295596 :`G` 0.037812 :`B` 0.34375 :`A` 1.0) 0.0)
  (`KismetSystemLibrary.PrintString` "Controls key :  \n- E for Interaction \n- N for No-Clip \n- G for Soul-Give" true false (struct :`R` 0.34375 :`G` 0.170933 :`A` 1.0) 0.0))

(event `EnhancedInput|/Game/ThirdParty/ThirdPerson/Input/Actions/IA_Interact`
  (params (ActionValue :type Boolean) (ElapsedSeconds :type "Float (double-precision)") (TriggeredSeconds :type "Float (double-precision)") (InputAction :type "InputAction Object Reference" :default "/Game/ThirdParty/ThirdPerson/Input/Actions/IA_Interact.IA_Interact"))
  (:`Triggered`
    (`self.InteractionKeyPressed`)))

(event `EnhancedInput|/Game/ThirdParty/ThirdPerson/Input/Actions/IA_SoulGive`
  (params (ActionValue :type Boolean) (ElapsedSeconds :type "Float (double-precision)") (TriggeredSeconds :type "Float (double-precision)") (InputAction :type "InputAction Object Reference" :default "/Game/ThirdParty/ThirdPerson/Input/Actions/IA_SoulGive.IA_SoulGive"))
  (:`Triggered`
    (`self.AddCollectable` "/Game/Blueprint/Collectable/SoulCollectable_BP.SoulCollectable_BP_C" 1)))

(fn `AddCollectable`
  (params (Collectable :type "/Game/Blueprint/Collectable/BaseCollectable_BP Class Reference") (Quantity :type Integer))
  (bind _inventory (`self.Inventory`))
  (`BlueprintMapLibrary.Map_Add` _inventory Collectable (+ (`BlueprintMapLibrary.Map_Find` _inventory Collectable) Quantity)))

(fn `ChangeCharacterMesh`
  (params (IsDead :type Boolean))
  (if IsDead
    (`MeshComponent.SetOverlayMaterial` (`self.Mesh`) "/Game/Material/VFXMaterials/M_Ghost_Overlay.M_Ghost_Overlay")
    (else
      (`MeshComponent.SetOverlayMaterial` (`self.Mesh`) null))))

(fn `ContainCollectable`
  (params (Collectable :type "/Game/Blueprint/Collectable/BaseCollectable_BP Class Reference"))
  (returns (IsContained :type Boolean))
  (return (`BlueprintMapLibrary.Map_Contains` (`self.Inventory`) Collectable)))

(fn `GetCollectable`
  (params (Collectable :type "/Game/Blueprint/Collectable/BaseCollectable_BP Class Reference"))
  (returns (Quantity :type Integer))
  (return (`BlueprintMapLibrary.Map_Find` (`self.Inventory`) Collectable)))

(fn `RemoveCollectable`
  (params (Collectable :type "/Game/Blueprint/Collectable/BaseCollectable_BP Class Reference") (Quantity :type Integer))
  (returns (IsRemoved :type Boolean))
  (if (>= (`self.GetCollectable` Collectable) Quantity)
    (bind _result (`/Engine/EditorBlueprintResources/StandardMacros.NegateInt` Quantity)
      (:`  `
        (`self.AddCollectable` Collectable _result)
        (return true)))
    (else
      (return false))))

(fn `UserConstructionScript`
  (`parent.UserConstructionScript`))

(fn `WorldSwich`
  (bind _output_get (set `self.IsInLivingWorld` (not (`self.IsInLivingWorld`))))
  (if _output_get
    (`self.K2_AddActorWorldOffset` (`self.WorldsSpacing`))
    (`self.ChangeCharacterMesh` false)
    (`self.LivingWorld`)
    (else
      (`self.K2_AddActorWorldOffset` (* (`self.WorldsSpacing`) -1))
      (`self.ChangeCharacterMesh` true)
      (`self.DeathWorld`))))