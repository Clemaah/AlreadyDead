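; Base activator Blueprint that lets the player fire an activation with the interaction key while inside its trigger box.
; Box overlap events bind OnInteract to the Character_BP's InteractionKeyPressed dispatcher on entry and clear all that dispatcher's bindings on exit.
; OnInteract calls the Activation dispatcher, then unbinds the key and overlap events if IsForUniqueUse is set.
; Debug strings trace entry, exit and repeatable presses.
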(event `self.ReceiveBeginPlay`
  (add `PrimitiveComponent.OnComponentBeginOverlap` (`self.Box`) (delegate `PlayerInRange`))
  (add `PrimitiveComponent.OnComponentEndOverlap` (`self.Box`) (delegate `PlayerOutOfRange`)))

(event `PlayerInRange`
  (params (OverlappedComponent :type "PrimitiveComponent Object Reference") (OtherActor :type "Actor Object Reference") (OtherComp :type "PrimitiveComponent Object Reference") (OtherBodyIndex :type Integer) (bFromSweep :type Boolean) (SweepResult :type "HitResult Structure (by ref)"))
  ;[1 1 1] Si le joueur rentre dans la zone de trigger, lier l'activable à l'événement d'appuie sur la touche d'interaction
  (bind _ascharacter_bp (cast `/Game/Blueprint/Character_BP` OtherActor))
  (add `/Game/Blueprint/Character_BP.InteractionKeyPressed` _ascharacter_bp (delegate `OnInteract`))
  (`KismetSystemLibrary.PrintString` "Je suis dans la box" true true (struct :`R` 0.489583 :`G` 0.398631 :`A` 1.0) 10.0))

(event `PlayerOutOfRange`
  (params (OverlappedComponent :type "PrimitiveComponent Object Reference") (OtherActor :type "Actor Object Reference") (OtherComp :type "PrimitiveComponent Object Reference") (OtherBodyIndex :type Integer))
  ;[1 1 1] Lorsque le joueur sort de la zone de trigger, délier l'activable de l'événement d'appui sur la touche d'interaction
  (bind _ascharacter_bp (cast `/Game/Blueprint/Character_BP` OtherActor))
  (clear `/Game/Blueprint/Character_BP.InteractionKeyPressed` _ascharacter_bp)
  (`KismetSystemLibrary.PrintString` "Je suis plus dans la box" true true (struct :`R` 0.489583 :`G` 0.398631 :`A` 1.0) 10.0))

(event `OnInteract`
  (`self.Activation`)
  ;[1 1 1] Délier l'événement à l'appui de la touche si l'activable est à usage unique
  (if (`self.IsForUniqueUse`)
    (clear `/Game/Blueprint/Character_BP.InteractionKeyPressed` (stale `PlayerInRange` _ascharacter_bp))
    (clear `PrimitiveComponent.OnComponentBeginOverlap` (`self.Box`))
    (clear `PrimitiveComponent.OnComponentEndOverlap` (`self.Box`))
    (else
      (`KismetSystemLibrary.PrintString` "J'ai appuyé" true true (struct :`R` 0.489583 :`G` 0.398631 :`A` 1.0) 10.0))))

(fn `UserConstructionScript`)