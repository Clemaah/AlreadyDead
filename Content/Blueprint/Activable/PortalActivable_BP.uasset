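; Interactable portal that, once paid for with souls, switches the player character between worlds.
; On interact, it tries to remove a set number of soul collectables from the player and only activates if that succeeds.
; Activation immediately switches a player already inside its box, runs the parent interact logic, then binds box overlap so later character entries also trigger the world switch.
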(event `self.OnInteract`
  (bind _returnvalue (`GameplayStatics.GetPlayerCharacter` 0))
  (bind _success (`self.TryActivate`))
  (if _success
    (`|ExecutionSequence`
      (:`then_0`
        (if (`PrimitiveComponent.IsOverlappingActor` (`self.Box`) _returnvalue)
          (bind _ascharacter_bp (cast `/Game/Blueprint/Character_BP` _returnvalue))
          (`self.Teleportation` _ascharacter_bp)))
      (:`then_1`
        (`parent.OnInteract`)
        (add `PrimitiveComponent.OnComponentBeginOverlap` (`self.Box`) (delegate `On Teleportation`))))))

(event `On Teleportation`
  (params (OverlappedComponent :type "PrimitiveComponent Object Reference") (OtherActor :type "Actor Object Reference") (OtherComp :type "PrimitiveComponent Object Reference") (OtherBodyIndex :type Integer) (bFromSweep :type Boolean) (SweepResult :type "HitResult Structure (by ref)"))
  (`self.Teleportation` OtherActor))

(fn `Teleportation`
  (params (Character :type "Actor Object Reference"))
  (bind _ascharacter_bp (cast `/Game/Blueprint/Character_BP` Character))
  (`/Game/Blueprint/Character_BP.WorldSwich` _ascharacter_bp))

(fn `TryActivate`
  (returns (Success :type Boolean))
  (bind _ascharacter_bp (cast `/Game/Blueprint/Character_BP` (`GameplayStatics.GetPlayerCharacter` 0)))
  (bind _isremoved (`/Game/Blueprint/Character_BP.RemoveCollectable` _ascharacter_bp "/Game/Blueprint/Collectable/SoulCollectable_BP.SoulCollectable_BP_C" (`self.NumberOfSouls`)))
  (return _isremoved))

(fn `UserConstructionScript`
  (`parent.UserConstructionScript`))