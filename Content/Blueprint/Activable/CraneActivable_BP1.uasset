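; An activable crane that rotates its Moveable component in yaw by a set angle when activated.
; A timeline drives the rotation, with play rate derived from separate forward and backward durations, and activation is ignored while rotating.
; Direction flips after each swing, and round-trip mode reverses automatically after a pause.
; The player character's death-world and living-world events stop and resume the animation.
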(event `self.ReceiveBeginPlay`
  (`parent.ReceiveBeginPlay`)
  (`self.SetAnimationDuration` (`self.ForwardDuration`))
  (bind _ascharacter_bp (cast `/Game/Blueprint/Character_BP` (`GameplayStatics.GetPlayerCharacter` 0)))
  (add `/Game/Blueprint/Character_BP.DeathWorld` _ascharacter_bp (delegate `Event OnPlayerDie`))
  (add `/Game/Blueprint/Character_BP.LivingWorld` _ascharacter_bp (delegate `Event OnPlayerRevive`)))

(event `Event OnPlayerDie`
  (`self.PauseAnimation`))

(event `Event OnPlayerRevive`
  (`self.UnpauseAnimation`))

(event `self.Activation`
  (`self.ActivateAnimation`))

(event `Event OnRoundTripReverse`
  (`KismetSystemLibrary.Delay` (`self.PauseDuration`))
  (bind (_direction _rotation) (`Timeline|Timeline` :!via `Reverse`)
    (:`Update`
      (`self.UpdateRotation` _rotation))
    (:`Finished`
      (`self.SwichTimelineDirection`)
      (if (and (not (`self.IsGoingForward`)) (`self.RoundTrip`))
        (`self.Event OnRoundTripReverse`)
        (else
          (set `self.IsRotating` false))))))

(fn `ActivateAnimation`
  (if (not (`self.IsRotating`))
    (set `self.IsRotating` true)
    (if (`self.IsGoingForward`)
      (`TimelineComponent.Play` (`self.Timeline`))
      (else
        (`TimelineComponent.Reverse` (`self.Timeline`))))))

(fn `PauseAnimation`
  (`TimelineComponent.Stop` (`self.Timeline`)))

(fn `SetAnimationDuration`
  (params (Duration :type "Float (double-precision)"))
  (`TimelineComponent.SetPlayRate` (`self.Timeline`) (/ 1.0 Duration)))

(fn `SwichTimelineDirection`
  (bind _output_get (set `self.IsGoingForward` (not (`self.IsGoingForward`))))
  (if _output_get
    (`self.SetAnimationDuration` (`self.ForwardDuration`))
    (else
      (`self.SetAnimationDuration` (`self.BackwardDuration`)))))

(fn `UnpauseAnimation`
  (if (`self.IsRotating`)
    (if (`self.IsGoingForward`)
      (`TimelineComponent.Play` (`self.Timeline`))
      (else
        (`TimelineComponent.Reverse` (`self.Timeline`))))))

(fn `UpdateRotation`
  (params (TimelineValue :type "Float (double-precision)"))
  (`SceneComponent.K2_SetRelativeRotation` (`self.Moveable`) (`KismetMathLibrary.RLerp` (struct) (`KismetMathLibrary.MakeRotator` 0.0 0.0 (`self.RotationAngle`)) TimelineValue true) false false))

(fn `UserConstructionScript`
  (`parent.UserConstructionScript`))