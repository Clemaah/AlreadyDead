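; GeneratorActivator_BP1 is an interactable button that removes a target actor from the level when used.
; On interact, it calls the parent logic, sets Pressed, moves the Button component down and plays a random click sound in 2D.
; It then destroys the actor referenced by Target, with no check of Pressed and no reset of the button within this graph.
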(event `self.OnInteract`
  (`parent.OnInteract`)
  (set `self.pressed` true)
  (`SceneComponent.K2_AddRelativeLocation` (`self.Button`) (0.0 0.0 -10.0) false false)
  (`GameplayStatics.PlaySound2D` "/Game/Sound/Mechanics/SC_RandomClick.SC_RandomClick" 1.0 1.0 0.0 null null)
  (`self.K2_DestroyActor` (`self.Target`)))

(fn `UserConstructionScript`
  (`parent.UserConstructionScript`))