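; DoorBase_BP is a base door that opens up once every attached locker is unlocked.
; On BeginPlay it gathers directly attached BaseLocker_BP actors, counts them and binds to their lock and unlock events.
; Lock events raise the counter and unlock events lower it.
; At zero it clears IsLock, blocks every locker and calls UnlockDoor, which is empty here, apparently for child doors to implement.
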(event `UnlockEventLocker`
  (bind _result (`/Engine/EditorBlueprintResources/StandardMacros.DecrementInt` (`self.CurrentLock`))
    (:`  `
      (if (== _result 0)
        (set `self.IsLock` false)
        (for _array_element (`self.Lockers`)
          (`/Game/Blueprint/TriggerPlayer/Locker/BaseLocker_BP.Block Lock` _array_element))
        (`self.Unlock Door`)))))

(event `self.ReceiveBeginPlay`
  (for _array_element (`self.GetAttachedActors` true)
    (bind _asbase_locker_bp (cast `/Game/Blueprint/TriggerPlayer/Locker/BaseLocker_BP` _array_element))
    (`/Engine/EditorBlueprintResources/StandardMacros.IncrementInt` (`self.NumberLocker`)
      (:`  `
        (`KismetArrayLibrary.Array_Add` (`self.Lockers`) _asbase_locker_bp)
        (add `/Game/Blueprint/TriggerPlayer/Locker/BaseLocker_BP.LockEvent` _asbase_locker_bp (delegate `LockEventLocker`))
        (add `/Game/Blueprint/TriggerPlayer/Locker/BaseLocker_BP.UnlockEvent` _asbase_locker_bp (delegate `UnlockEventLocker`)))))
  (set `self.CurrentLock` (`self.NumberLocker`)))

(event `LockEventLocker`
  (`/Engine/EditorBlueprintResources/StandardMacros.IncrementInt` (`self.CurrentLock`)))

(event `Unlock Door`)

(fn `UserConstructionScript`)