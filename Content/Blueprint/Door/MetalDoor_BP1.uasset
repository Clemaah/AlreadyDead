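; A metal door Blueprint that slides its two parts, Haut (top) and Bas (bottom), open when unlocked.
; UnlockDoor calls the parent implementation, then starts one timeline per part through a sequence, so both move together.
; Each timeline lerps its part's world location toward a marker component, Sphere or Sphere1, restarting from the current position every update rather than a stored start point.
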(event `self.Unlock Door`
  (bind _haut (`self.Haut`))
  (bind _bas (`self.Bas`))
  (`parent.Unlock Door`)
  (`|ExecutionSequence`
    (:`then_0`
      (bind (_direction _newtrack_0) (`Timeline|Timeline`)
        (:`Update`
          (`SceneComponent.K2_SetWorldLocation` _haut (`KismetMathLibrary.VLerp` (`SceneComponent.K2_GetComponentLocation` _haut) (`SceneComponent.K2_GetComponentLocation` (`self.Sphere`)) _newtrack_0) false false))))
    (:`then_1`
      (bind (_direction_2 _newtrack_0_2) (`Timeline|Timeline_0`)
        (:`Update`
          (`SceneComponent.K2_SetWorldLocation` _bas (`KismetMathLibrary.VLerp` (`SceneComponent.K2_GetComponentLocation` _bas) (`SceneComponent.K2_GetComponentLocation` (`self.Sphere1`)) _newtrack_0_2) false false))))))

(fn `UserConstructionScript`
  (`parent.UserConstructionScript`))