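; MetalDoor_BP is a two-piece sliding door that opens when unlocked, extending a parent door Blueprint.
; UnlockDoor calls the parent version, then starts two timelines that move Cube and Cube1 toward the Sphere and Sphere1 target markers.
; Each update lerps from the piece's current location rather than a stored start, so the motion compounds instead of following the curve linearly.
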(event `self.Unlock Door`
  (bind _cube (`self.Cube`))
  (bind _cube1 (`self.Cube1`))
  (`parent.Unlock Door`)
  (`|ExecutionSequence`
    (:`then_0`
      (bind (_direction _newtrack_0) (`Timeline|Timeline` :`NewTime` 0.0)
        (:`Update`
          (`SceneComponent.K2_SetWorldLocation` _cube (`KismetMathLibrary.VLerp` (`SceneComponent.K2_GetComponentLocation` _cube) (`SceneComponent.K2_GetComponentLocation` (`self.Sphere`)) _newtrack_0) false false))))
    (:`then_1`
      (bind (_direction_2 _newtrack_0_2) (`Timeline|Timeline_0` :`NewTime` 0.0)
        (:`Update`
          (`SceneComponent.K2_SetWorldLocation` _cube1 (`KismetMathLibrary.VLerp` (`SceneComponent.K2_GetComponentLocation` _cube1) (`SceneComponent.K2_GetComponentLocation` (`self.Sphere1`)) _newtrack_0_2) false false))))))

(fn `UserConstructionScript`
  (`parent.UserConstructionScript`))