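; A moving platform that travels to a target point while the player stands on it and returns when they leave.
; Overlaps of CollisionSphere with Character_BP toggle a flag that selects TargetSphere or TargetSphere1 as the destination.
; Every Tick, the Cylinder moves toward that sphere's current world location at constant Speed using VInterpToConstant, without sweep.
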(event `self.CollisionSphere.OnComponentBeginOverlap`
  (params (OverlappedComponent :type "PrimitiveComponent Object Reference") (OtherActor :type "Actor Object Reference") (OtherComp :type "PrimitiveComponent Object Reference") (OtherBodyIndex :type Integer) (bFromSweep :type Boolean) (SweepResult :type "HitResult Structure (by ref)"))
  ;[1 1 1] Activate / Desactivate the variable when the player enter/leave the sphere collision
  (cast `/Game/Blueprint/Character_BP` OtherActor)
  (set `self.PlayerOnPlateform` true))

(event `self.CollisionSphere.OnComponentEndOverlap`
  (params (OverlappedComponent :type "PrimitiveComponent Object Reference") (OtherActor :type "Actor Object Reference") (OtherComp :type "PrimitiveComponent Object Reference") (OtherBodyIndex :type Integer))
  ;[1 1 1] Activate / Desactivate the variable when the player enter/leave the sphere collision
  (cast `/Game/Blueprint/Character_BP` OtherActor)
  (set `self.PlayerOnPlateform` false))

(event `self.ReceiveBeginPlay`
  ;[1 1 1] Define the two positions of the plateform (initial and target point)
  (set `self.Target` (`SceneComponent.K2_GetComponentLocation` (`self.TargetSphere`)))
  (set `self.Target2` (`SceneComponent.K2_GetComponentLocation` (`self.TargetSphere1`))))

(event `self.ReceiveTick`
  (params (DeltaSeconds :type "Float (single-precision)"))
  ;[1 1 1] Move the plateform to the target point (if player is on the plateform) or move it back to initial position if not already there
  (if (`self.PlayerOnPlateform`)
    (set `self.Target` (`SceneComponent.K2_GetComponentLocation` (`self.TargetSphere`)))
    (else
      (set `self.Target` (`SceneComponent.K2_GetComponentLocation` (`self.TargetSphere1`)))))
  (`SceneComponent.K2_SetWorldLocation` (`self.Cylinder`) (`KismetMathLibrary.VInterpTo_Constant` (`SceneComponent.K2_GetComponentLocation` (`self.Cylinder`)) (`self.Target`) (`GameplayStatics.GetWorldDeltaSeconds`) (`self.speed`)) false false))

(fn `UserConstructionScript`)