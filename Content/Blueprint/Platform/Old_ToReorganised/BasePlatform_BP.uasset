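; Base moving platform that slides its GroupMove component between its start position and a Target marker, only while the player character is in the living world.
; Tick drives constant-speed interpolation; on arrival, after a delay, it either reverses with a per-direction speed or switches ticking off.
; Ticking doubles as the on/off switch, set by StartImmediatly and EnablePlatform.
; ApplyArrow stretches a cylinder between GroupMove and Target to show the path.
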(event `self.ReceiveBeginPlay`
  (set `self.TargetLocation` (`SceneComponent.K2_GetComponentLocation` (`self.Target`)))
  (set `self.StartLocation` (`SceneComponent.K2_GetComponentLocation` (`self.Group Move`)))
  (`self.SetActorTickEnabled` (`self.StartImmediatly`)))

(event `self.ReceiveTick`
  (params (DeltaSeconds :type "Float (single-precision)"))
  (bind _ascharacter_bp (cast `/Game/Blueprint/Character_BP` (`GameplayStatics.GetPlayerCharacter` 0)))
  (if (`/Game/Blueprint/Character_BP.IsInLivingWorld` _ascharacter_bp)
    (bind _newposition (`self.MovePlatform` DeltaSeconds (`self.TargetLocation`)))
    (`SceneComponent.K2_SetWorldLocation` (`self.Group Move`) _newposition false true)
    (if (== (`self.TargetLocation`) _newposition)
      (`KismetSystemLibrary.Delay` (`self.Delay`))
      (if (`self.Loop`)
        (`self.Reverse Target`)
        (else
          (`self.SetActorTickEnabled` false))))))

(fn `ApplyArrow`
  (bind _cylinder (`self.Cylinder`))
  (bind _returnvalue (- (`SceneComponent.K2_GetComponentLocation` (`self.Target`)) (`SceneComponent.K2_GetComponentLocation` (`self.Group Move`))))
  (`SceneComponent.K2_SetWorldLocationAndRotation` _cylinder (+ (`SceneComponent.K2_GetComponentLocation` (`self.Group Move`)) (/ _returnvalue (2.0 2.0 2.0))) (`KismetMathLibrary.Conv_VectorToRotator` _returnvalue) false true)
  (`SceneComponent.K2_AddRelativeRotation` _cylinder (struct :`Pitch` 90.0) false false)
  (`SceneComponent.SetWorldScale3D` _cylinder (`KismetMathLibrary.MakeVector` 0.1 0.1 (/ (`KismetMathLibrary.VSize` _returnvalue) 100.0))))

(fn `EnablePlatform`
  (params (enable :type Boolean))
  (`self.SetActorTickEnabled` enable))

(fn `MovePlatform`
  (params (deltaTime :type "Float (double-precision)") (target :type "Vector Structure"))
  (returns (newPosition :type "Vector Structure"))
  (return (`KismetMathLibrary.VInterpTo_Constant` (`SceneComponent.K2_GetComponentLocation` (`self.Group Move`)) target deltaTime (`self.Speed`))))

(fn `Reverse Target`
  (if (== (`self.TargetLocation`) (`SceneComponent.K2_GetComponentLocation` (`self.Target`)))
    (set `self.TargetLocation` (`self.StartLocation`))
    (set `self.Speed` (`self.SpeedBack`))
    (else
      (set `self.TargetLocation` (`SceneComponent.K2_GetComponentLocation` (`self.Target`)))
      (set `self.Speed` (`self.SpeedForward`)))))

(fn `UserConstructionScript`)