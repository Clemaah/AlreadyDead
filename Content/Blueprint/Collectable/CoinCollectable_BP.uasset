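; CoinCollectable_BP is a coin collectable Blueprint that animates its Cylinder component, with no pickup logic in its graphs.
; Each Tick sets the cylinder's relative Z from GetNewLocation and adds RotationSpeed as yaw, without delta-time scaling.
; GetNewLocation holds a time-based sine bob using MovementSpeed and MovementAmplitude, but that expression is marked unused.
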(event `self.ReceiveTick`
  (params (DeltaSeconds :type "Float (single-precision)"))
  (`SceneComponent.K2_SetRelativeLocation` (`self.Cylinder`) (`KismetMathLibrary.MakeVector` 0.0 0.0 (* (`KismetMathLibrary.Sin` (* (`GameplayStatics.GetTimeSeconds`) (`self.MovementSpeed`))) (`self.MovementAmplitude`))) false false)
  (`SceneComponent.K2_AddRelativeRotation` (`self.Cylinder`) (`KismetMathLibrary.MakeRotator` 0.0 0.0 (`self.RotationSpeed`)) false false))

(fn `UserConstructionScript`
  (`parent.UserConstructionScript`))