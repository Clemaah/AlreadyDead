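; RespawnTest_BP is a trigger Blueprint, apparently for testing respawn, that gives visual confirmation when triggered by a player.
; It extends a parent's EventTrigger, calling the parent logic first and then making Cube1 visible.
; If the referenced TextRenderer is valid, it turns that text green and sets it to "Activated".
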(event `self.ReceiveBeginPlay`
  (`parent.ReceiveBeginPlay`))

(event `/Game/Blueprint/TriggerPlayer/TriggerPlayer_BP.Event trigger`
  (params (player :type "/Game/Blueprint/Character_BP Object Reference"))
  (bind _textrender (`TextRenderActor.TextRender` (`self.TextRenderer`)))
  (`parent.Event trigger` player)
  (`SceneComponent.SetVisibility` (`self.Cube1`) true false)
  (`/Engine/EditorBlueprintResources/StandardMacros.IsValid` (`self.TextRenderer`)
    (:`Is Valid`
      (`TextRenderComponent.SetTextRenderColor` _textrender (make `Color` 0 255 0 255))
      (`TextRenderComponent.K2_SetText` _textrender "Activated"))))

(fn `UserConstructionScript`
  (`parent.UserConstructionScript`))