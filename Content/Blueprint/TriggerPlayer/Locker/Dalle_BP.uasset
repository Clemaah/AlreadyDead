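; Dalle_BP is a tile actor in the player-trigger locker set that shows a locked or unlocked state through its color.
; BeginPlay creates a dynamic material instance from the Cube's first material, sets it to the lock color and applies it to the Cube.
; The Lock and Unlock events only switch that instance's Color parameter between the lock and unlock colors.
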(event `self.ReceiveBeginPlay`
  (`parent.ReceiveBeginPlay`)
  (bind _returnvalue (`KismetMaterialLibrary.CreateDynamicMaterialInstance` (`PrimitiveComponent.GetMaterial` (`self.Cube`) 0)))
  (bind _output_get (set `self.Mat` _returnvalue))
  (`MaterialInstanceDynamic.SetVectorParameterValue` _output_get "Color" (`self.LockColor`))
  (`PrimitiveComponent.SetMaterial` (`self.Cube`) 0 (`self.Mat`)))

(event `self.Lock`
  (`MaterialInstanceDynamic.SetVectorParameterValue` (`self.Mat`) "Color" (`self.LockColor`)))

(event `self.Unlock`
  (`MaterialInstanceDynamic.SetVectorParameterValue` (`self.Mat`) "Color" (`self.UnlockColor`)))

(fn `UserConstructionScript`
  (`parent.UserConstructionScript`))