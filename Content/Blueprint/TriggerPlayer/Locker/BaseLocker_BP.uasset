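; BaseLocker_BP is a base locker Blueprint that unlocks when triggered and can relock itself after a timer.
; EventTrigger acts only while locked: it clears IsLock, records the start time, then calls CallUnlockEvent and the empty Unlock hook.
; With UseTimer on, it waits for Timer, then restores the lock through CallLockEvent and the empty Lock hook.
; BlockLock sets TotalyLocked, which cancels that timed relock.
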(event `self.ReceiveBeginPlay`
  (`parent.ReceiveBeginPlay`))

(event `self.Event trigger`
  (params (player :type "/Game/Blueprint/Character_BP Object Reference"))
  (if (`self.IsLock`)
    (set `self.IsLock` false)
    (set `self.StartTimer` (`GameplayStatics.GetTimeSeconds`))
    (`self.UnlockEvent`)
    (`self.Unlock`)
    (if (`self.UseTimer`)
      (`KismetSystemLibrary.Delay` (`self.Timer`))
      (if (not (`self.TotalyLocked`))
        (set `self.IsLock` true)
        (`self.LockEvent`)
        (`self.Lock`)))))

(event `Unlock`)

(event `Lock`)

(fn `Block Lock`
  (set `self.TotalyLocked` true))

(fn `UserConstructionScript`
  (`parent.UserConstructionScript`))