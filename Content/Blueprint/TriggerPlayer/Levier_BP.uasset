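; Lever trigger that rotates a target crane actor when something overlaps its box.
; The lever timeline tilts the pivot and plays the crane timeline, then reverses a second after overlap ends.
; Tick pauses the crane while the player character is outside the living world and resumes it on return.
; When the crane timeline finishes, it reverses after a one-second delay.
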(event `self.ReceiveTick`
  (params (DeltaSeconds :type "Float (single-precision)"))
  (if (`self.CraneAnim`)
    (bind _ascharacter_bp (cast `/Game/Blueprint/Character_BP` (`GameplayStatics.GetPlayerCharacter` 0)))
    (if (`/Game/Blueprint/Character_BP.IsInLivingsWorld` _ascharacter_bp)
      (if (`self.pauseAnim`)
        (set `self.pauseAnim` false)
        (bind (_direction _gruerotation) (`Timeline|CraneTimeline` :!label _label)
          (:`Update`
            (set `self.CraneAnim` true)
            (bind _ascharacter_bp_2 (cast `/Game/Blueprint/Character_BP` (`GameplayStatics.GetPlayerCharacter` 0)))
            (if (`/Game/Blueprint/Character_BP.IsInLivingsWorld` _ascharacter_bp_2)
              (`SceneComponent.K2_SetRelativeRotation` (`Actor.RootComponent` (`self.TargetActor`)) (`KismetMathLibrary.RLerp` (struct) (`self.EndRotationGrue`) _gruerotation true) false false)))
          (:`Finished`
            (set `self.CraneAnim` false)
            (`self.EndAnimation`))))
      (else
        (set `self.pauseAnim` true)
        (goto _label :!via `Stop`)))))

(event `self.Box.OnComponentBeginOverlap`
  (params (OverlappedComponent :type "PrimitiveComponent Object Reference") (OtherActor :type "Actor Object Reference") (OtherComp :type "PrimitiveComponent Object Reference") (OtherBodyIndex :type Integer) (bFromSweep :type Boolean) (SweepResult :type "HitResult Structure (by ref)"))
  (if (not (`self.LeverAnim`))
    (bind (_direction _leverrotation) (`Timeline|LeverTimeline` :!label _label_2)
      (:`Update`
        (set `self.LeverAnim` true)
        (`SceneComponent.K2_SetRelativeRotation` (`self.Pivot`) (`KismetMathLibrary.RLerp` (struct) (`self.EndRotationLever`) _leverrotation true) false false)
        (goto _label))
      (:`Finished`
        (set `self.LeverAnim` false)))))

(event `EndAnimation`
  (`KismetSystemLibrary.Delay` 1.0)
  (goto _label :!via `Reverse`))

(event `self.Box.OnComponentEndOverlap`
  (params (OverlappedComponent :type "PrimitiveComponent Object Reference") (OtherActor :type "Actor Object Reference") (OtherComp :type "PrimitiveComponent Object Reference") (OtherBodyIndex :type Integer))
  (`KismetSystemLibrary.Delay` 1.0)
  (goto _label_2 :!via `Reverse`))

(fn `UserConstructionScript`)