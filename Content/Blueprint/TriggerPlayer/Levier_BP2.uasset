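; Lever that, on box overlap, swings its pivot and rotates a linked target actor, advancing the target's end rotation 90 degrees after each completed turn.
; Separate timelines drive lever and target, with the lever reversing after a two-second delay.
; Tick pauses the target's rotation while the player is outside the living world and resumes it on return.
; Death and living world events are bound to Character_BP but left empty.
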(event `self.ReceiveBeginPlay`
  (bind _ascharacter_bp (cast `/Game/Blueprint/Character_BP` (`GameplayStatics.GetPlayerCharacter` 0)))
  (add `/Game/Blueprint/Character_BP.DeathWorld` _ascharacter_bp (delegate `DeathWorld`))
  (add `/Game/Blueprint/Character_BP.LivingWorld` _ascharacter_bp (delegate `LivingWorld`)))

(event `DeathWorld`)

(event `LivingWorld`)

(event `self.ReceiveTick`
  (params (DeltaSeconds :type "Float (single-precision)"))
  (if (`self.ObjectAnim`)
    (bind _ascharacter_bp (cast `/Game/Blueprint/Character_BP` (`GameplayStatics.GetPlayerCharacter` 0)))
    (if (`/Game/Blueprint/Character_BP.IsInLivingWorld` _ascharacter_bp)
      (if (`self.PauseAnim`)
        (set `self.PauseAnim` false)
        (bind (_direction _gruerotation) (`Timeline|ObjectTimeline` :!label _label)
          (:`Update`
            (set `self.ObjectAnim` true)
            (`SceneComponent.K2_SetWorldRotation` (`Actor.RootComponent` (`self.TargetActor`)) (`KismetMathLibrary.RLerp` (`self.StartRotationTarget`) (`self.EndRotationTarget`) _gruerotation true) false false))
          (:`Finished`
            (set `self.ObjectAnim` false)
            (set `self.EndRotationTarget` (`KismetMathLibrary.ComposeRotators` (`self.EndRotationTarget`) (struct :`Yaw` 90.0))))))
      (else
        (set `self.PauseAnim` true)
        (goto _label :!via `Stop`)))))

(event `self.Box.OnComponentBeginOverlap`
  (params (OverlappedComponent :type "PrimitiveComponent Object Reference") (OtherActor :type "Actor Object Reference") (OtherComp :type "PrimitiveComponent Object Reference") (OtherBodyIndex :type Integer) (bFromSweep :type Boolean) (SweepResult :type "HitResult Structure (by ref)"))
  (if (not (`self.LeverAnim`))
    (`|ExecutionSequence`
      (:`then_0`
        (bind (_direction _leverrotation) (`Timeline|LeverTimeline` :!label _label_2)
          (:`Update`
            (set `self.LeverAnim` true)
            (`SceneComponent.K2_SetRelativeRotation` (`self.Pivot`) (`KismetMathLibrary.RLerp` (struct) (`self.EndRotationLever`) _leverrotation true) false false))
          (:`Finished`
            (set `self.LeverAnim` false))))
      (:`then_1`
        (`KismetSystemLibrary.Delay` 2.0)
        (goto _label_2 :!via `Reverse`))
      (:`then_2`
        (set `self.StartRotationTarget` (`self.K2_GetActorRotation` (`self.TargetActor`)))
        (goto _label :!via `PlayFromStart`)))))

(fn `UserConstructionScript`)